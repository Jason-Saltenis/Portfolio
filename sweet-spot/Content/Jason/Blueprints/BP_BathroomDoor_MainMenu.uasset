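; BP_BathroomDoor_MainMenu is an interactable bathroom door that swings open and closed with sound effects.
; CanInteract lets a first-person character through if the door needs no keycard color or the character's keycard matches it.
; A successful interaction toggles DoorStatus and plays or reverses a Timeline that yaws the Pivot, with door collision disabled until it finishes.
; A failed interaction only plays a knob rattle.
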(event `self.InteractSuccess`
  (params (InteractingCaller :type "Actor Object Reference"))
  (`PrimitiveComponent.SetCollisionEnabled` (`self.BathroomDoor`) "NoCollision")
  (switch `/Game/Jason/Enums/En_DoorStatus` (`self.DoorStatus`)
    (:`NewEnumerator0`
      (`FMODBlueprintStatics.PlayEventAtLocation` "/Game/FMOD/Events/Door/Door_Open_Creak.Door_Open_Creak" (`KismetMathLibrary.Conv_VectorToTransform` (`self.K2_GetActorLocation` self)))
      (set `self.DoorStatus` "NewEnumerator1")
      (bind (_direction _door_float) (`Timeline|Timeline` :!label _label)
        (:`Update`
          (`SceneComponent.K2_SetRelativeRotation` (`self.pivot`) (`KismetMathLibrary.MakeRotator` 0.0 0.0 _door_float) false false))
        (:`Finished`
          (`PrimitiveComponent.SetCollisionEnabled` (`self.BathroomDoor`) "QueryAndPhysics"))))
    (:`NewEnumerator1`
      (`FMODBlueprintStatics.PlayEventAtLocation` "/Game/FMOD/Events/Door/Door_Wood_Close.Door_Wood_Close" (`KismetMathLibrary.Conv_VectorToTransform` (`self.K2_GetActorLocation` self)))
      (set `self.DoorStatus` "NewEnumerator0")
      (goto _label :!via `Reverse`))))

(event `self.InteractFail`
  (params (`Interacting Actor` :type "Actor Object Reference"))
  (`FMODBlueprintStatics.PlayEventAtLocation` "/Game/FMOD/Events/Door/Door_Knob_Rattle.Door_Knob_Rattle" (`KismetMathLibrary.Conv_VectorToTransform` (`self.K2_GetActorLocation` self))))

(fn `CanInteract`
  (params (InteractingActor :type "Actor Object Reference"))
  (returns (CanInteract :type Boolean))
  (bind _doorcolor (`self.DoorColor`))
  (bind _asbp_first_person_character (cast `/Game/FirstPerson/Blueprints/BP_FirstPersonCharacter` InteractingActor))
  (if (== _doorcolor (struct))
    _
    (elif (== (`/Game/FirstPerson/Blueprints/BP_FirstPersonCharacter.KeycardColor` _asbp_first_person_character) _doorcolor)
      _
      (else
        (return false))))
  (return true))

(fn `UserConstructionScript`)