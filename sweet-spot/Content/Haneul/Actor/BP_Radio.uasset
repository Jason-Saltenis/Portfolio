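; BP_Radio is an interactable radio actor that the first-person player can switch on and off.
; On BeginPlay it plays or stops its Radio component according to the IsPlaying flag.
; Each successful interaction toggles playback and flips that flag, while CanInteract allows only BP_FirstPersonCharacter to interact.
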(event `self.ReceiveBeginPlay`
  (bind _radio (`self.Radio`))
  (if (`self.isPlaying`)
    (`FMODAudioComponent.Play` _radio)
    (else
      (`FMODAudioComponent.Stop` _radio))))

(event `/Game/Jason/Interface/BPI_InteractInterface.InteractSuccess`
  (params (InteractingCaller :type "Actor Object Reference"))
  (bind _radio (`self.Radio`))
  (bind _returnvalue (not (`self.isPlaying`)))
  (if (`self.isPlaying`)
    (`FMODAudioComponent.Stop` _radio)
    (set `self.isPlaying` _returnvalue)
    (else
      (`FMODAudioComponent.Play` _radio)
      (set `self.isPlaying` _returnvalue))))

(fn `CanInteract`
  (params (InteractingActor :type "Actor Object Reference"))
  (returns (CanInteract :type Boolean))
  (cast `/Game/FirstPerson/Blueprints/BP_FirstPersonCharacter` InteractingActor)
  (return true))

(fn `UserConstructionScript`)