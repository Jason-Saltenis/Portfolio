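; BP_FadeObject fades the SaneActors and SweetActors groups in or out by animating material opacity.
; Fade stores start values and per-tick steps, then starts two 0.1-second looping timers that run until opacity reaches either limit.
; Each tick creates dynamic material instances on mesh components to set Opacity.
; Sweet actors also toggle visibility and collision, with BP_TeleportDoor meshes using a temporary material during the fade and wood once visible.
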(event `self.Fade`
  (params (saneTime :type "Float (single-precision)") (saneStartValue :type "Float (single-precision)") (sweetTime :type "Float (single-precision)") (sweetStartValue :type "Float (single-precision)"))
  (set `self.SaneTime` saneTime)
  (set `self.SaneCurrentValue` saneStartValue)
  (set `self.SweetTime` sweetTime)
  (set `self.SweetCurrentValue` sweetStartValue)
  (bind _returnvalue (`KismetSystemLibrary.K2_SetTimerDelegate` (delegate `CustomEvent`) 0.1 true))
  (set `self.TimerHandle` _returnvalue)
  (bind _returnvalue_2 (`KismetSystemLibrary.K2_SetTimerDelegate` (delegate `CustomEvent_0`) 0.1 true))
  (set `self.TimerHandle2` _returnvalue_2)
  (for _array_element (`self.SweetActors`)
    (`/Engine/EditorBlueprintResources/StandardMacros.IsValid` _array_element
      (:`Is Valid`
        (`Actor.SetActorHiddenInGame` _array_element false)
        (for _array_element_2 (`Actor.K2_GetComponentsByClass` _array_element "/Script/Engine.StaticMeshComponent")
          (`PrimitiveComponent.SetCollisionEnabled` _array_element_2 "QueryAndPhysics")
          (cast `/Game/Haneul/Actor/BP_TeleportDoor` _array_element)
          (if (not (== (`self.SweetTime`) 0.0))
            (`PrimitiveComponent.SetMaterial` _array_element_2 1 "/Game/Haneul/MAT_Brown.MAT_Brown")
            (if (== (`self.SweetCurrentValue`) 0.0)
              (bind _returnvalue_3 (`PrimitiveComponent.CreateDynamicMaterialInstance` _array_element_2 1 (`PrimitiveComponent.GetMaterial` _array_element_2 1) "None"))
              (`MaterialInstanceDynamic.SetScalarParameterValue` _returnvalue_3 "Opacity" 0.0))))))))

(event `CustomEvent`
  (bind _newparam (`self.Fadeing`))
  (if _newparam
    (bind _output_get (set `self.TimerHandle` (struct)))
    (`KismetSystemLibrary.K2_ClearAndInvalidateTimerHandle` _output_get)))

(event `CustomEvent_0`
  (bind _newparam (`self.Fading2`))
  (if _newparam
    (bind _output_get (set `self.TimerHandle2` (struct)))
    (`KismetSystemLibrary.K2_ClearAndInvalidateTimerHandle` _output_get)
    (if (<= (`self.SweetCurrentValue`) 0.0)
      (for _array_element (`self.SweetActors`)
        (`/Engine/EditorBlueprintResources/StandardMacros.IsValid` _array_element
          (:`Is Valid`
            (`Actor.SetActorHiddenInGame` _array_element true)
            (for _array_element_2 (`Actor.K2_GetComponentsByClass` _array_element "/Script/Engine.StaticMeshComponent")
              (`PrimitiveComponent.SetCollisionEnabled` _array_element_2 "NoCollision")))))
      (else
        (for _array_element_3 (`self.SweetActors`)
          (for _array_element_4 (`Actor.K2_GetComponentsByClass` _array_element_3 "/Script/Engine.StaticMeshComponent")
            (cast `/Game/Haneul/Actor/BP_TeleportDoor` _array_element_3)
            (`PrimitiveComponent.SetMaterial` _array_element_4 1 "/Game/Game/Art/Environments/TilingTextures/Hotel_Furniture_Wood/MI_WoodFurniture.MI_WoodFurniture")))))))

(fn `Fadeing`
  (returns (NewParam :type Boolean))
  (bind _output_get (set `self.SaneCurrentValue` (+ (`self.SaneTime`) (`self.SaneCurrentValue`))))
  (for _array_element (`self.SaneActors`)
    (`/Engine/EditorBlueprintResources/StandardMacros.IsValid` _array_element
      (:`Is Valid`
        (bind _returnvalue (`Actor.K2_GetComponentsByClass` _array_element "/Script/Engine.StaticMeshComponent"))
        (if (!= (`KismetArrayLibrary.Array_Length` _returnvalue) 0)
          (for (_ _array_index) _returnvalue
            (bind _output (`|GetArrayItem` _returnvalue _array_index))
            (for (_array_element_2 _array_index_2) (`MeshComponent.GetMaterials` _output)
              (bind _returnvalue_2 (`PrimitiveComponent.CreateDynamicMaterialInstance` _output _array_index_2 _array_element_2 "None"))
              (`PrimitiveComponent.SetMaterial` _output 0 _returnvalue_2)
              (`MaterialInstanceDynamic.SetScalarParameterValue` _returnvalue_2 "Opacity" (`self.SaneCurrentValue`))))
          (else
            (for _array_element_3 (`Actor.K2_GetComponentsByClass` _array_element "/Script/Engine.SkeletalMeshComponent")
              (for (_array_element_4 _array_index_3) (`MeshComponent.GetMaterials` _array_element_3)
                (bind _returnvalue_3 (`PrimitiveComponent.CreateDynamicMaterialInstance` _array_element_3 _array_index_3 _array_element_4 "None"))
                (`PrimitiveComponent.SetMaterial` _array_element_3 0 _returnvalue_3)
                (`MaterialInstanceDynamic.SetScalarParameterValue` _returnvalue_3 "Opacity" (`self.SaneCurrentValue`)))))))))
  (return (or (>= _output_get 1.0) (<= _output_get 0.0))))

(fn `Fading2`
  (returns (NewParam :type Boolean))
  (bind _output_get (set `self.SweetCurrentValue` (+ (`self.SweetTime`) (`self.SweetCurrentValue`))))
  (for _array_element (`self.SweetActors`)
    (`/Engine/EditorBlueprintResources/StandardMacros.IsValid` _array_element
      (:`Is Valid`
        (bind _returnvalue (`Actor.K2_GetComponentsByClass` _array_element "/Script/Engine.StaticMeshComponent"))
        (for (_ _array_index) _returnvalue
          (bind _output (`|GetArrayItem` _returnvalue _array_index))
          (for (_array_element_2 _array_index_2) (`MeshComponent.GetMaterials` _output)
            (bind _returnvalue_2 (`PrimitiveComponent.CreateDynamicMaterialInstance` _output _array_index_2 _array_element_2 "None"))
            (`MaterialInstanceDynamic.SetScalarParameterValue` _returnvalue_2 "Opacity" (`self.SweetCurrentValue`))
            (for _array_element_3 (`Actor.K2_GetComponentsByClass` _array_element "/Script/Engine.SkeletalMeshComponent")
              (for (_array_element_4 _array_index_3) (`MeshComponent.GetMaterials` _array_element_3)
                (bind _returnvalue_3 (`PrimitiveComponent.CreateDynamicMaterialInstance` _array_element_3 _array_index_3 _array_element_4 "None"))
                (`MaterialInstanceDynamic.SetScalarParameterValue` _returnvalue_3 "Opacity" (`self.SweetCurrentValue`)))))))))
  (return (or (>= _output_get 1.0) (<= _output_get 0.0))))