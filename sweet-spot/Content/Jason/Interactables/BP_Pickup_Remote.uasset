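; Interactable remote pickup in a chained puzzle, where only the active remote is highlighted through custom depth stencil and can be collected.
; Collecting it destroys it along with the smoke and smoke trigger actors, then activates the next remote or reveals the hidden keycard, and turns on the linked TV.
; Picking an inactive remote raises the madness meter, shakes the camera, plays a sound and briefly flashes a jump-scare widget.
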(event `self.ReceiveBeginPlay`
  (bind _key (`self.Key`))
  (bind _remote (`self.Remote`))
  (`self.RedFlash`)
  (`/Engine/EditorBlueprintResources/StandardMacros.IsValid` _key
    (:`Is Valid`
      (`self.SetActorEnableCollision` _key false)
      (`self.SetActorHiddenInGame` _key true))
    (:`Is Not Valid`
      _))
  (if (`self.Active`)
    (`PrimitiveComponent.SetCustomDepthStencilValue` _remote 1)
    (else
      (`PrimitiveComponent.SetCustomDepthStencilValue` _remote 0))))

(event `/Game/Jason/Interface/BPI_InteractInterface.InteractSuccess`
  (params (InteractingCaller :type "Actor Object Reference"))
  (bind _nextremote (`self.NextRemote`))
  (bind _tv (`self.TV`))
  (bind _key (`self.Key`))
  (if (`self.Active`)
    (`FMODBlueprintStatics.PlayEventAtLocation` "/Game/FMOD/Events/UI/ButtonMouseOver.ButtonMouseOver" (`KismetMathLibrary.Conv_VectorToTransform` (`self.K2_GetActorLocation` self)))
    (bind _returnvalue (`GameplayStatics.GetActorOfClass` "/Game/Jason/Blueprints/BP_Smoke.BP_Smoke_C"))
    (bind _returnvalue_2 (`GameplayStatics.GetActorOfClass` "/Game/Jason/Blueprints/BP_TriggerSmoke.BP_TriggerSmoke_C"))
    (`self.K2_DestroyActor` self)
    (`self.K2_DestroyActor` _returnvalue)
    (`self.K2_DestroyActor` _returnvalue_2)
    (`/Engine/EditorBlueprintResources/StandardMacros.IsValid` _nextremote
      (:`Is Valid`
        (set `/Game/Jason/Interactables/BP_Pickup_Remote.Active` true _nextremote)
        (`PrimitiveComponent.SetCustomDepthStencilValue` (`/Game/Jason/Interactables/BP_Pickup_Remote.Remote` _nextremote) 1))
      (:`Is Not Valid`
        (`/Engine/EditorBlueprintResources/StandardMacros.IsValid` _key
          (:`Is Valid`
            (`self.SetActorEnableCollision` _key true)
            (`self.SetActorHiddenInGame` _key false)
            (`PrimitiveComponent.SetCustomDepthStencilValue` (`/Game/Jason/Interactables/BP_Keycard.Keycard` _key) 1)))))
    (`/Engine/EditorBlueprintResources/StandardMacros.IsValid` _tv
      (:`Is Valid`
        (`/Game/Haneul/Actor/BP_ToggleableTV.TurnTVOn` _tv)))
    (else
      (`self.IncreaseMadness`)
      (`self.CameraShake`)
      (`FMODBlueprintStatics.PlayEventAtLocation` null (`KismetMathLibrary.Conv_VectorToTransform` (`self.K2_GetActorLocation` self)))
      (set `Widget.Visibility` "Visible" (`self.redFlashWidget`))
      (`KismetSystemLibrary.Delay` 0.2)
      (set `Widget.Visibility` "Hidden" (`self.redFlashWidget`)))))

(fn `CameraShake`
  (`GameplayStatics.PlayWorldCameraShake` null (`self.K2_GetActorLocation` (`Controller.K2_GetPawn` (`GameplayStatics.GetPlayerController` 0))) 0.0 1000.0))

(fn `CanInteract`
  (params (InteractingActor :type "Actor Object Reference"))
  (returns (CanInteract :type Boolean))
  (cast `/Game/FirstPerson/Blueprints/BP_FirstPersonCharacter` InteractingActor)
  (return true))

(fn `IncreaseMadness`
  (bind _asplayer_hud (cast `PlayerHud` (`PlayerController.GetHUD` (`GameplayStatics.GetPlayerController` 0))))
  (bind _asbp_madness_bar (cast `/Game/Jason/UI/Blueprints/BP_MadnessBar` (`PlayerHud.GetMadnessMeterWidget` _asplayer_hud)))
  (`MyUserWidget.IncreaseMadnessBar` _asbp_madness_bar (`self.Increase Madness`)))

(fn `RedFlash`
  (bind _returnvalue (`|CreateWidget` "/Game/Haneul/Widget/WBP_JumpScare.WBP_JumpScare_C"))
  (bind _output_get (set `self.redFlashWidget` _returnvalue))
  (`UserWidget.AddToViewport` _output_get 0)
  (set `Widget.Visibility` "Hidden" (`self.redFlashWidget`)))

(fn `UserConstructionScript`)