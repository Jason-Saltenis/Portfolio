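; Numbered room door (301–306) that opens and closes through interaction, gated by the player's keycard color.
; A timeline rotates door and handle with FMOD sounds, while the construction script picks the nameplate mesh and sizes trigger boxes.
; Room 304 enlarges the HUD key pop-up on overlap until first successful interaction.
; An optional closing trigger shuts an open door behind the player and changes its required color to Lock.
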(event `self.ReceiveBeginPlay`
  (`KismetSystemLibrary.DelayUntilNextTick`)
  (if (`|EnumEquality` (`self.Number`) "NewEnumerator3")
    (bind _asplayer_hud (cast `PlayerHud` (`PlayerController.GetHUD` (`GameplayStatics.GetPlayerController` 0))))
    (bind _aswbp_pop_up (cast `/Game/Haneul/Widget/WBP_PopUp` (`PlayerHud.PopUpWidget` _asplayer_hud)))
    (set `self.PopUpWidget` _aswbp_pop_up)))

(event `LockDoor`
  (switch `/Game/Jason/Enums/En_DoorStatus` (`self.DoorStatus`) :!label _label
    (:`NewEnumerator0`
      (`FMODBlueprintStatics.PlayEventAtLocation` "/Game/FMOD/Events/Foley/OpenDoor.OpenDoor" (`SceneComponent.K2_GetComponentToWorld` (`self.FRAME`)))
      (set `self.DoorStatus` "NewEnumerator1")
      (bind (_direction _door_float _doorknob_float) (`Timeline|Timeline` :!label _label_2)
        (:`Update`
          (`SceneComponent.K2_SetRelativeRotation` (`self.DOOR`) (`KismetMathLibrary.MakeRotator` 0.0 0.0 _door_float) false false)
          (`SceneComponent.K2_SetRelativeRotation` (`self.HandleScene`) (`KismetMathLibrary.MakeRotator` _doorknob_float) false false))
        (:`Finished`
          (`PrimitiveComponent.SetCollisionEnabled` (`self.DOOR`) "QueryAndPhysics"))))
    (:`NewEnumerator1`
      (`FMODBlueprintStatics.PlayEventAtLocation` "/Game/FMOD/Events/SFX/DoorClose.DoorClose" (`SceneComponent.K2_GetComponentToWorld` (`self.FRAME`)))
      (set `self.DoorStatus` "NewEnumerator0")
      (goto _label_2 :!via `Reverse`))))

(event `self.InteractSuccess`
  (params (InteractingCaller :type "Actor Object Reference"))
  (`self.CheckIf304`)
  (`PrimitiveComponent.SetCollisionEnabled` (`self.DOOR`) "NoCollision")
  (goto _label))

(event `self.InteractFail`
  (params (`Interacting Actor` :type "Actor Object Reference"))
  (`FMODBlueprintStatics.PlayEventAtLocation` "/Game/FMOD/Events/SFX/DoorLock.DoorLock" (`KismetMathLibrary.Conv_VectorToTransform` (`self.K2_GetActorLocation` self))))

(event `self.304Box.OnComponentBeginOverlap`
  (params (OverlappedComponent :type "PrimitiveComponent Object Reference") (OtherActor :type "Actor Object Reference") (OtherComp :type "PrimitiveComponent Object Reference") (OtherBodyIndex :type Integer) (bFromSweep :type Boolean) (SweepResult :type "HitResult Structure (by ref)"))
  (bind _popupwidget (`self.PopUpWidget`))
  (cast `/Game/FirstPerson/Blueprints/BP_FirstPersonCharacter` OtherActor)
  (cast `CapsuleComponent` OtherComp)
  (`/Engine/EditorBlueprintResources/StandardMacros.IsValid` _popupwidget
    (:`Is Valid`
      (`/Game/Haneul/Widget/WBP_PopUp.KeyPopUpSize` _popupwidget 1.4))))

(event `self.304Box.OnComponentEndOverlap`
  (params (OverlappedComponent :type "PrimitiveComponent Object Reference") (OtherActor :type "Actor Object Reference") (OtherComp :type "PrimitiveComponent Object Reference") (OtherBodyIndex :type Integer))
  (bind _popupwidget (`self.PopUpWidget`))
  (cast `/Game/FirstPerson/Blueprints/BP_FirstPersonCharacter` OtherActor)
  (cast `CapsuleComponent` OtherComp)
  (`/Engine/EditorBlueprintResources/StandardMacros.IsValid` _popupwidget
    (:`Is Valid`
      (`/Game/Haneul/Widget/WBP_PopUp.KeyPopUpSize` _popupwidget 1.0))))

(event `self.ClosingDoorBox.OnComponentBeginOverlap`
  (params (OverlappedComponent :type "PrimitiveComponent Object Reference") (OtherActor :type "Actor Object Reference") (OtherComp :type "PrimitiveComponent Object Reference") (OtherBodyIndex :type Integer) (bFromSweep :type Boolean) (SweepResult :type "HitResult Structure (by ref)"))
  (if (`self.ClosingTrigger`)
    (cast `/Game/FirstPerson/Blueprints/BP_FirstPersonCharacter` OtherActor)
    (cast `CapsuleComponent` OtherComp)
    (if (`|EnumEquality` (`self.DoorStatus`) "NewEnumerator1")
      (`self.LockDoor`)
      (set `self.DoorColor` (struct :`TagName` "SweetSpot.KeyCard.Color.Lock")))))

(fn `CanInteract`
  (params (InteractingActor :type "Actor Object Reference"))
  (returns (CanInteract :type Boolean))
  (bind _doorcolor (`self.DoorColor`))
  (bind _asbp_first_person_character (cast `/Game/FirstPerson/Blueprints/BP_FirstPersonCharacter` InteractingActor))
  (if (== _doorcolor (struct))
    _
    (elif (== (`/Game/FirstPerson/Blueprints/BP_FirstPersonCharacter.KeycardColor` _asbp_first_person_character) _doorcolor)
      _
      (else
        (return false))))
  (return true))

(fn `CheckIf304`
  (bind _304box (`self.304Box`))
  (`/Engine/EditorBlueprintResources/StandardMacros.IsValid` _304box
    (:`Is Valid`
      (`ActorComponent.K2_DestroyComponent` _304box))))

(fn `CloseDoor`
  (set `self.DoorStatus` "NewEnumerator1")
  (set `self.DoorColor` (struct :`TagName` "SweetSpot.KeyCard.Color.Lock"))
  (`self.LockDoor`))

(fn `OpenDoor`
  (set `self.DoorStatus` "NewEnumerator0")
  (`self.LockDoor`))

(fn `UserConstructionScript`
  (`BoxComponent.SetBoxExtent` (`self.304Box`) (0.0 0.0 0.0) true)
  (`BoxComponent.SetBoxExtent` (`self.ClosingDoorBox`) (0.0 0.0 0.0) true)
  (if (`self.ClosingTrigger`)
    (`BoxComponent.SetBoxExtent` (`self.ClosingDoorBox`) (100.0 100.0 100.0) true))
  (switch `/Game/Haneul/DoorNumber` (`self.Number`)
    (:`NewEnumerator0`
      (`StaticMeshComponent.SetStaticMesh` (`self.NamePlate_301`) "/Game/Game/Art/Environments/Man-Made/Props/Furniture/NamePlate_301.NamePlate_301"))
    (:`NewEnumerator1`
      (`StaticMeshComponent.SetStaticMesh` (`self.NamePlate_301`) "/Game/Game/Art/Environments/Man-Made/Props/Furniture/NamePlate_302.NamePlate_302"))
    (:`NewEnumerator2`
      (`StaticMeshComponent.SetStaticMesh` (`self.NamePlate_301`) "/Game/Game/Art/Environments/Man-Made/Props/Furniture/NamePlate_303.NamePlate_303"))
    (:`NewEnumerator3`
      (`StaticMeshComponent.SetStaticMesh` (`self.NamePlate_301`) "/Game/Game/Art/Environments/Man-Made/Props/Furniture/NamePlate_304.NamePlate_304")
      (`BoxComponent.SetBoxExtent` (`self.304Box`) (150.0 150.0 150.0) true))
    (:`NewEnumerator4`
      (`StaticMeshComponent.SetStaticMesh` (`self.NamePlate_301`) "/Game/Game/Art/Environments/Man-Made/Props/Furniture/NamePlate_305.NamePlate_305"))
    (:`NewEnumerator5`
      (`StaticMeshComponent.SetStaticMesh` (`self.NamePlate_301`) "/Game/Game/Art/Environments/Man-Made/Props/Furniture/NamePlate_306.NamePlate_306"))))