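; BP_ShowTentacle is a trigger actor that reveals an array of tentacle actors while the first-person character's capsule overlaps its collision component.
; The tentacles start hidden at BeginPlay, show on begin overlap and hide again on end overlap.
; Showing and hiding toggle visibility and collision on each entry and its nested Tentacle actor, call Spawn or StartDown, and play or stop the tentacle sound.
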(event `self.ReceiveBeginPlay`
  (`self.HideTentacle`))

(event `self.CollisionComponent.OnComponentBeginOverlap`
  (params (OverlappedComponent :type "PrimitiveComponent Object Reference") (OtherActor :type "Actor Object Reference") (OtherComp :type "PrimitiveComponent Object Reference") (OtherBodyIndex :type Integer) (bFromSweep :type Boolean) (SweepResult :type "HitResult Structure (by ref)"))
  (cast `CapsuleComponent` OtherComp)
  (cast `/Game/FirstPerson/Blueprints/BP_FirstPersonCharacter` OtherActor)
  (`self.ShowTentacle`))

(event `self.CollisionComponent.OnComponentEndOverlap`
  (params (OverlappedComponent :type "PrimitiveComponent Object Reference") (OtherActor :type "Actor Object Reference") (OtherComp :type "PrimitiveComponent Object Reference") (OtherBodyIndex :type Integer))
  (cast `CapsuleComponent` OtherComp)
  (cast `/Game/FirstPerson/Blueprints/BP_FirstPersonCharacter` OtherActor)
  (`self.HideTentacle`))

(fn `HideTentacle`
  (for _array_element (`self.Tentacle`)
    (`/Engine/EditorBlueprintResources/StandardMacros.IsValid` _array_element
      (:`Is Valid`
        (bind _rootcomponent (`Actor.RootComponent` _array_element))
        (`/Engine/EditorBlueprintResources/StandardMacros.IsValid` _rootcomponent
          (:`Is Valid`
            (`SceneComponent.SetVisibility` _rootcomponent false true)
            (`SceneComponent.SetVisibility` (`Actor.RootComponent` (`/Game/Haneul/Actor/BP_TentacleWall.Tentacle` _array_element)) false true)
            (`self.SetActorEnableCollision` _array_element false)
            (`self.SetActorEnableCollision` (`/Game/Haneul/Actor/BP_TentacleWall.Tentacle` _array_element) false)
            (`TentacleWall.StartDown` _array_element)
            (`FMODAudioComponent.Stop` (`/Game/Harnoorr/BP/BP_NEW/BP_TENTACLE.SFX_Tenticle` (`/Game/Haneul/Actor/BP_TentacleWall.Tentacle` _array_element)))))))))

(fn `ShowTentacle`
  (for _array_element (`self.Tentacle`)
    (`/Engine/EditorBlueprintResources/StandardMacros.IsValid` _array_element
      (:`Is Valid`
        (`SceneComponent.SetVisibility` (`Actor.RootComponent` _array_element) true true)
        (`SceneComponent.SetVisibility` (`Actor.RootComponent` (`/Game/Haneul/Actor/BP_TentacleWall.Tentacle` _array_element)) true true)
        (`self.SetActorEnableCollision` _array_element true)
        (`self.SetActorEnableCollision` (`/Game/Haneul/Actor/BP_TentacleWall.Tentacle` _array_element) true)
        (`TentacleWall.Spawn` _array_element)
        (`FMODAudioComponent.Play` (`/Game/Harnoorr/BP/BP_NEW/BP_TENTACLE.SFX_Tenticle` (`/Game/Haneul/Actor/BP_TentacleWall.Tentacle` _array_element)))))))

(fn `UserConstructionScript`)