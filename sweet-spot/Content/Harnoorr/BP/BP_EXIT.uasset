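; Exit sign actor that, when switched on, seals the level's doors and starts a flickering light.
; TurnLightOn runs once, lighting the spotlight, playing FMOD audio, closing the door nearest the player and setting door colors to locked.
; It closes other doors on staggered, randomized timers and locks test doors with their triggers disabled.
; A looping timer randomly blacks out the spotlight, darkens sign meshes and schedules the spotlight's restore.
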(fn `CloseClostestDoor`
  (bind _outactors (`GameplayStatics.GetAllActorsOfClass` "/Game/Harnoorr/BP/BP_NEW/BP_NEW_DOOR_COPY.BP_NEW_DOOR_COPY_C"))
  (for _array_element _outactors
    (bind _returnvalue (`KismetMathLibrary.Vector_Distance` (`SceneComponent.K2_GetComponentLocation` (`/Game/Harnoorr/BP/BP_NEW/BP_NEW_DOOR_COPY.NamePlate_301` _array_element)) (`self.K2_GetActorLocation` (`GameplayStatics.GetPlayerPawn` 0))))
    (if (< _returnvalue (`self.closestDoor`))
      (set `self.closestDoor` _returnvalue)
      (set `self.ClosestDoorActor` _array_element)))
  (`/Game/Harnoorr/BP/BP_NEW/BP_NEW_DOOR_COPY.CloseDoor` (`self.ClosestDoorActor`)))

(fn `FlickerLight`
  (bind _array (`|MakeArray` (`self.TR-BL`) (`self.Top`) (`self.Mid`) (`self.Back`) (`self.Top-down`) (`self.Top-down1`) (`self.Block`) (`self.Tri`) (`self.TL-BR`) (`self.Bottom`) (`self.TL-BR1`) (`self.TL-BR2`) (`self.TL-BR3`) (`self.TL-BR5`) (`self.TL-BR6`) (`self.TL-BR7`) (`self.TL-BR4`) (`self.TL-BR8`) (`self.Letter-I`)))
  (if (> (`KismetMathLibrary.RandomFloatInRange` 0.0 1.0) 0.5)
    (`LightComponent.SetIntensity` (`self.SpotLight`) 0.0)
    (`KismetSystemLibrary.K2_SetTimer` null "Light" 0.1 false false 0.05)
    (if (`self.isOn`)
      (for _array_element _array
        (`MeshComponent.SetColorParameterValueOnMaterials` _array_element "ExitSignColor" (struct :`R` 0.005208 :`G` 0.005208 :`B` 0.005208 :`A` 1.0)))
      (else
        (for _array_element_2 _array
          (`MeshComponent.SetColorParameterValueOnMaterials` _array_element_2 "ExitSignColor" (struct :`R` 1.0 :`A` 1.0)))))))

(fn `Light`
  (bind _spotlight (`self.SpotLight`))
  (`LocalLightComponent.SetAttenuationRadius` _spotlight 500.0)
  (`LightComponent.SetIntensity` _spotlight 50.0))

(fn `TurnLightOn`
  (if (not (`self.isOn`))
    (`self.Light`)
    (`self.CloseClostestDoor`)
    (`FMODBlueprintStatics.PlayEventAtLocation` "/Game/FMOD/Events/SFX/Exit_Sign.Exit_Sign" (`SceneComponent.K2_GetComponentToWorld` (`self.FMODAudio1`)))
    (bind _outactors (`GameplayStatics.GetAllActorsOfClass` "/Game/Harnoorr/BP/BP_NEW/BP_NEW_DOOR_COPY.BP_NEW_DOOR_COPY_C"))
    (for _array_element _outactors
      (set `/Game/Harnoorr/BP/BP_NEW/BP_NEW_DOOR_COPY.DoorColor` (struct :`TagName` "SweetSpot.KeyCard.Color.Lock") _array_element)
      (if (not (`|EnumEquality` (`/Game/Harnoorr/BP/BP_NEW/BP_NEW_DOOR_COPY.DoorStatus` _array_element) "NewEnumerator0"))
        (`KismetSystemLibrary.K2_SetTimer` _array_element "CloseDoor" 0.5 false false (`self.Initial Start Delay`) 1.0)
        (set `self.Initial Start Delay` (+ (`self.Initial Start Delay`) 0.1))))
    (bind _outactors_2 (`GameplayStatics.GetAllActorsOfClass` "/Game/Harnoorr/BP/BP_NEW/BP_TEST_DOOR.BP_TEST_DOOR_C"))
    (for _array_element_2 _outactors_2
      (`PrimitiveComponent.SetCollisionEnabled` (`/Game/Harnoorr/BP/BP_NEW/BP_TEST_DOOR.OpenDoorTriggerbox` _array_element_2) "NoCollision")
      (`/Game/Harnoorr/BP/BP_NEW/BP_TEST_DOOR.LockDoor` _array_element_2 "NewEnumerator0"))
    (set `self.isOn` true)
    (`KismetSystemLibrary.K2_SetTimer` null "FlickerLight" 0.2 true)))

(fn `UserConstructionScript`)