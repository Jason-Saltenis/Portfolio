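; BP_OpenDoor is a one-shot trigger actor that fires a linked TeleportDoor when the player walks into it.
; On collision overlap it accepts only the capsule component of BP_FirstPersonCharacter.
; If the door reference is valid, its Status is the first enum value and it is not hidden, the trigger calls InteractSuccess on the door, then destroys itself.
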(event `self.CollisionComponent.OnComponentBeginOverlap`
  (params (OverlappedComponent :type "PrimitiveComponent Object Reference") (OtherActor :type "Actor Object Reference") (OtherComp :type "PrimitiveComponent Object Reference") (OtherBodyIndex :type Integer) (bFromSweep :type Boolean) (SweepResult :type "HitResult Structure (by ref)"))
  (bind _teleportdoor (`self.TeleportDoor`))
  (`/Engine/EditorBlueprintResources/StandardMacros.IsValid` (`self.TeleportDoor`)
    (:`Is Valid`
      (cast `CapsuleComponent` OtherComp)
      (cast `/Game/FirstPerson/Blueprints/BP_FirstPersonCharacter` OtherActor)
      (if (`|EnumEquality` (`/Game/Haneul/Actor/BP_TeleportDoor.Status` (`self.TeleportDoor`)) "NewEnumerator0")
        (if (not (`Actor.bHidden` _teleportdoor))
          (`/Game/Jason/Interface/BPI_InteractInterface.InteractSuccess` _teleportdoor null)
          (`self.K2_DestroyActor`))))))

(fn `UserConstructionScript`)