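; Trigger actor that spawns a BP_TentacleWall at BeginPlay, hidden and inactive, and reveals it when a character walks in.
; The wall attaches to the SpawnTentacle component with a pitch offset and receives this actor's madness and speed settings.
; A capsule overlap on TriggerBox calls TentacleFadeIn to enable visibility, collision, movement and sound, then disables the trigger and opens linked doors.
; EndPlay destroys the tentacle.
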(event `self.ReceiveBeginPlay`
  (bind _spawntentacle (`self.spawnTentacle`))
  (bind _tentacle (`self.Tentacle`))
  (`/Engine/EditorBlueprintResources/StandardMacros.IsValid` _spawntentacle
    (:`Is Valid`
      (bind _returnvalue (`|SpawnActorFromClass` "/Game/Haneul/Actor/BP_TentacleWall.BP_TentacleWall_C" (`KismetMathLibrary.MakeTransform` (`SceneComponent.K2_GetComponentLocation` _spawntentacle) (`KismetMathLibrary.MakeRotator` 0.0 (+ (.pitch (`SceneComponent.RelativeRotation` _spawntentacle)) -90.0) (.yaw (`SceneComponent.RelativeRotation` _spawntentacle)))) "AlwaysSpawn" "MultiplyWithRoot" null null))
      (bind _output_get (set `self.Tentacle` _returnvalue))
      (`self.K2_AttachToComponent` _output_get (`self.spawnTentacle`) "None" "KeepWorld" "KeepWorld" "KeepWorld" true)
      (`self.TentacleFadeIn` false)
      ; set up tentacle
      (set `TentacleWall.IncreaseMadness` (`self.IncreaseMadness`) _tentacle)
      (set `TentacleWall.comingUpSpeed` (`self.comingUpSpeed`) _tentacle)
      (set `TentacleWall.restoreMadnessValue` (`self.restoreMadnessValue`) _tentacle)
      (set `TentacleWall.MadnessTickInterval` (`self.MadnessTickInterval`) _tentacle)
      (set `TentacleWall.isActive` false (`self.Tentacle`))
      (`FMODAudioComponent.SetPaused` (`/Game/Harnoorr/BP/BP_NEW/BP_TENTACLE.SFX_Tenticle` (`/Game/Haneul/Actor/BP_TentacleWall.Tentacle` (`self.Tentacle`))) true))))

(event `self.triggerBox.OnComponentBeginOverlap`
  (params (OverlappedComponent :type "PrimitiveComponent Object Reference") (OtherActor :type "Actor Object Reference") (OtherComp :type "PrimitiveComponent Object Reference") (OtherBodyIndex :type Integer) (bFromSweep :type Boolean) (SweepResult :type "HitResult Structure (by ref)"))
  (cast `Character` OtherActor)
  (cast `CapsuleComponent` OtherComp)
  (`self.TentacleFadeIn` true)
  (`PrimitiveComponent.SetCollisionEnabled` (`self.triggerBox`) "NoCollision")
  (for _array_element (`self.DoorToOpen`)
    (`/Engine/EditorBlueprintResources/StandardMacros.IsValid` _array_element
      (:`Is Valid`
        (`/Game/Harnoorr/BP/BP_NEW/BP_OLD_DOOR.OpenDoor` _array_element)))))

(event `self.ReceiveEndPlay`
  (params (EndPlayReason :type "EEndPlayReason Enum" :default "Destroyed"))
  (bind _tentacle (`self.Tentacle`))
  (`/Engine/EditorBlueprintResources/StandardMacros.IsValid` _tentacle
    (:`Is Valid`
      (`/Game/Haneul/Actor/BP_TentacleWall.Destroy Tentacle` _tentacle))))

(fn `TentacleFadeIn`
  (params (isFadingIn :type Boolean))
  (bind _tentacle (`self.Tentacle`))
  (bind _tentacle_2 (`/Game/Haneul/Actor/BP_TentacleWall.Tentacle` (`self.Tentacle`)))
  (bind _box (`/Game/Harnoorr/BP/BP_NEW/BP_TENTACLE.Box` _tentacle_2))
  (`SceneComponent.SetHiddenInGame` (`/Game/Harnoorr/BP/BP_NEW/BP_TENTACLE.SkeletalMesh` _tentacle_2) (not isFadingIn) false)
  (`SceneComponent.SetHiddenInGame` (`Actor.RootComponent` (`self.Tentacle`)) (not isFadingIn) false)
  (`SceneComponent.SetHiddenInGame` (`/Game/Haneul/Actor/BP_TentacleWall.Sphere` (`self.Tentacle`)) (not isFadingIn) false)
  (`SceneComponent.SetHiddenInGame` (`/Game/Haneul/Actor/BP_TentacleWall.Cone` (`self.Tentacle`)) (not isFadingIn) false)
  (`SceneComponent.SetHiddenInGame` (`/Game/Haneul/Actor/BP_TentacleWall.NS_Vortex_Base` (`self.Tentacle`)) (not isFadingIn) false)
  (`SceneComponent.SetHiddenInGame` (`/Game/Haneul/Actor/BP_TentacleWall.NS_Vortex` (`self.Tentacle`)) (not isFadingIn) false)
  (if isFadingIn
    (`PrimitiveComponent.SetCollisionEnabled` _box "QueryAndPhysics")
    (`PrimitiveComponent.SetCollisionEnabled` (`TentacleWall.triggerBox` (`self.Tentacle`)) "QueryAndPhysics")
    (`TentacleWall.StartDown` _tentacle)
    (`TentacleWall.Spawn` _tentacle)
    (set `TentacleWall.isActive` true _tentacle)
    (`FMODAudioComponent.SetPaused` (`/Game/Harnoorr/BP/BP_NEW/BP_TENTACLE.SFX_Tenticle` (`/Game/Haneul/Actor/BP_TentacleWall.Tentacle` (`self.Tentacle`))) false)
    (else
      (`PrimitiveComponent.SetCollisionEnabled` _box "NoCollision")
      (`PrimitiveComponent.SetCollisionEnabled` (`TentacleWall.triggerBox` (`self.Tentacle`)) "NoCollision")
      (`FMODAudioComponent.SetPaused` (`/Game/Harnoorr/BP/BP_NEW/BP_TENTACLE.SFX_Tenticle` (`/Game/Haneul/Actor/BP_TentacleWall.Tentacle` (`self.Tentacle`))) true))))

(fn `UserConstructionScript`)