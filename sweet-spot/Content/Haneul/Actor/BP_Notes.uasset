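; BP_Notes is a readable note pickup that the first-person character can interact with.
; The construction script uses a per-instance Notes selection to set the plane's material and matching page texture.
; On a successful interaction it passes itself and the texture to the HUD's WBP_PopUp as an instruction prompt.
; It then hides itself and disables the plane's collision.
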(event `/Game/Jason/Interface/BPI_InteractInterface.InteractSuccess`
  (params (InteractingCaller :type "Actor Object Reference"))
  (bind _asplayer_hud (cast `PlayerHud` (`PlayerController.GetHUD` (`GameplayStatics.GetPlayerController` 0))))
  (bind _aswbp_pop_up (cast `/Game/Haneul/Widget/WBP_PopUp` (`PlayerHud.PopUpWidget` _asplayer_hud)))
  (set `/Game/Haneul/Widget/WBP_PopUp.NoteActor` self _aswbp_pop_up)
  (bind _astexture_2d (cast `Texture2D` (`self.Text`)))
  (`/Game/Haneul/Widget/WBP_PopUp.Prompt` _aswbp_pop_up _astexture_2d true (1.0 1.41))
  (`self.SetActorHiddenInGame` true)
  (`PrimitiveComponent.SetCollisionEnabled` (`self.Plane`) "NoCollision"))

(fn `CanInteract`
  (params (InteractingActor :type "Actor Object Reference"))
  (returns (CanInteract :type Boolean))
  (cast `/Game/FirstPerson/Blueprints/BP_FirstPersonCharacter` InteractingActor)
  (return true))

(fn `UserConstructionScript`
  (bind _plane (`self.Plane`))
  (switch `/Game/Haneul/Notes` (`self.Notes`)
    (:`NewEnumerator0`
      (`PrimitiveComponent.SetMaterial` _plane 0 "/Game/Game/Art/Environments/Man-Made/Props/Furniture/Materials/Notes/MI_Notes.MI_Notes")
      (set `self.Text` "/Game/Jason/UI/HUDArt/Notes/Note1.Note1"))
    (:`NewEnumerator1`
      (`PrimitiveComponent.SetMaterial` _plane 0 "/Game/Game/Art/Environments/Man-Made/Props/Furniture/Materials/Notes/MI_Notes02.MI_Notes02")
      (set `self.Text` "/Game/Jason/UI/HUDArt/Notes/Note2.Note2"))
    (:`NewEnumerator2`
      (`PrimitiveComponent.SetMaterial` _plane 0 "/Game/Game/Art/Environments/Man-Made/Props/Furniture/Materials/Notes/MI_Notes03.MI_Notes03")
      (set `self.Text` "/Game/Jason/UI/HUDArt/Notes/Note3.Note3"))
    (:`NewEnumerator3`
      (`PrimitiveComponent.SetMaterial` _plane 0 "/Game/Game/Art/Environments/Man-Made/Props/Furniture/Materials/Notes/MI_Notes04.MI_Notes04")
      (set `self.Text` "/Game/Jason/UI/HUDArt/Notes/Note4.Note4"))
    (:`NewEnumerator4`
      (`PrimitiveComponent.SetMaterial` _plane 0 "/Game/Game/Art/Environments/Man-Made/Props/Furniture/Materials/Notes/MI_Notes05.MI_Notes05")
      (set `self.Text` "/Game/Jason/UI/HUDArt/Notes/Note5.Note5"))
    (:`NewEnumerator5`
      (`PrimitiveComponent.SetMaterial` _plane 0 "/Game/Game/Art/Environments/Man-Made/Props/Furniture/Materials/Notes/MI_Notes06.MI_Notes06")
      (set `self.Text` "/Game/Jason/UI/HUDArt/Notes/Note6.Note6"))
    (:`NewEnumerator6`
      (`PrimitiveComponent.SetMaterial` _plane 0 "/Game/Game/Art/Environments/Man-Made/Props/Furniture/Materials/Notes/MI_Notes07.MI_Notes07")
      (set `self.Text` "/Game/Jason/UI/HUDArt/Notes/Note7.Note7"))
    (:`NewEnumerator7`
      (`PrimitiveComponent.SetMaterial` _plane 0 "/Game/Game/Art/Environments/Man-Made/Props/Furniture/Materials/Notes/MI_Notes08.MI_Notes08")
      (set `self.Text` "/Game/Jason/UI/HUDArt/Notes/Note8.Note8"))
    (:`NewEnumerator8`
      (`PrimitiveComponent.SetMaterial` _plane 0 "/Game/Game/Art/Environments/Man-Made/Props/Furniture/Materials/Notes/MI_Notes09.MI_Notes09")
      (set `self.Text` "/Game/Jason/UI/HUDArt/Notes/Note9.Note9"))
    (:`NewEnumerator9`
      (`PrimitiveComponent.SetMaterial` _plane 0 "/Game/Game/Art/Environments/Man-Made/Props/Furniture/Materials/Notes/MI_Notes10.MI_Notes10")
      (set `self.Text` "/Game/Jason/UI/HUDArt/Notes/Note10.Note10"))
    (:`NewEnumerator10`
      (`PrimitiveComponent.SetMaterial` _plane 0 "/Game/Game/Art/Environments/Man-Made/Props/Furniture/Materials/Notes/MI_Notes11.MI_Notes11")
      (set `self.Text` "/Game/Jason/UI/HUDArt/Notes/Note11.Note11"))))