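; Keycard-gated room door that swings open or shut and sets its numbered nameplate mesh (301–306) in the construction script.
; Interaction requires a matching keycard color and an unlocked state, then toggles a timeline that rotates door and knob with sound, disabling door collision while moving.
; Failed attempts on a closed door rattle the knob sound.
; Character-capsule trigger boxes force open or closed via LockDoor; the close box starts with collision disabled.
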(event `self.ReceiveBeginPlay`
  (`PrimitiveComponent.SetCollisionEnabled` (`self.CloseDoorTriggerbox`) "NoCollision"))

(event `CloseDoor`
  (`PrimitiveComponent.SetCollisionEnabled` (`self.DOOR`) "NoCollision" :!label _label)
  (switch `/Game/Jason/Enums/En_DoorStatus` (`self.DoorStatus`)
    (:`NewEnumerator0`
      (`FMODBlueprintStatics.PlayEventAtLocation` "/Game/FMOD/Events/Foley/OpenDoor.OpenDoor" (`KismetMathLibrary.Conv_VectorToTransform` (`self.K2_GetActorLocation` self)))
      (set `self.DoorStatus` "NewEnumerator1")
      (bind (_direction _door_float _doorknob_float) (`Timeline|Timeline` :!label _label_2)
        (:`Update`
          (`SceneComponent.K2_SetRelativeRotation` (`self.DOOR`) (`KismetMathLibrary.MakeRotator` 0.0 0.0 _door_float) false false)
          (`SceneComponent.K2_SetRelativeRotation` (`self.HandleScene`) (`KismetMathLibrary.MakeRotator` _doorknob_float) false false))
        (:`Finished`
          (`PrimitiveComponent.SetCollisionEnabled` (`self.DOOR`) "QueryAndPhysics"))))
    (:`NewEnumerator1`
      (`FMODBlueprintStatics.PlayEventAtLocation` "/Game/FMOD/Events/SFX/DoorClose.DoorClose" (`KismetMathLibrary.Conv_VectorToTransform` (`self.K2_GetActorLocation` self)))
      (set `self.DoorStatus` "NewEnumerator0")
      (goto _label_2 :!via `Reverse`))))

(event `/Game/Jason/Interface/BPI_InteractInterface.InteractSuccess`
  (params (InteractingCaller :type "Actor Object Reference"))
  (goto _label))

(event `self.OpenDoorTriggerbox.OnComponentBeginOverlap`
  (params (OverlappedComponent :type "PrimitiveComponent Object Reference") (OtherActor :type "Actor Object Reference") (OtherComp :type "PrimitiveComponent Object Reference") (OtherBodyIndex :type Integer) (bFromSweep :type Boolean) (SweepResult :type "HitResult Structure (by ref)"))
  (cast `Character` OtherActor)
  (cast `CapsuleComponent` OtherComp)
  (`self.LockDoor` "NewEnumerator1"))

(event `self.CloseDoorTriggerbox.OnComponentBeginOverlap`
  (params (OverlappedComponent :type "PrimitiveComponent Object Reference") (OtherActor :type "Actor Object Reference") (OtherComp :type "PrimitiveComponent Object Reference") (OtherBodyIndex :type Integer) (bFromSweep :type Boolean) (SweepResult :type "HitResult Structure (by ref)"))
  (cast `Character` OtherActor)
  (cast `CapsuleComponent` OtherComp)
  (`self.LockDoor` "NewEnumerator0"))

(event `self.InteractFail`
  (params (`Interacting Actor` :type "Actor Object Reference"))
  (if (`|EnumEquality` (`self.DoorStatus`) "NewEnumerator0")
    (`FMODBlueprintStatics.PlayEventAtLocation` "/Game/FMOD/Events/Door/Door_Knob_Rattle.Door_Knob_Rattle" (`KismetMathLibrary.Conv_VectorToTransform` (`self.K2_GetActorLocation` self)))))

(fn `CanInteract`
  (params (InteractingActor :type "Actor Object Reference"))
  (returns (CanInteract :type Boolean))
  (bind _asbp_first_person_character (cast `/Game/FirstPerson/Blueprints/BP_FirstPersonCharacter` InteractingActor))
  (return (and (== (`/Game/FirstPerson/Blueprints/BP_FirstPersonCharacter.KeycardColor` _asbp_first_person_character) (`self.DoorColor`)) (not (`self.isLocked`)))))

(fn `LockDoor`
  (params (lock :type "/Game/Jason/Enums/En_DoorStatus Enum" :default "NewEnumerator0"))
  (if (not (`|EnumEquality` lock (`self.DoorStatus`)))
    (`self.CloseDoor`)))

(fn `UserConstructionScript`
  (switch `/Game/Haneul/DoorNumber` (`self.Number`)
    (:`NewEnumerator0`
      (`StaticMeshComponent.SetStaticMesh` (`self.Name Plate 301`) "/Game/Game/Art/Environments/Man-Made/Props/Furniture/NamePlate_301.NamePlate_301"))
    (:`NewEnumerator1`
      (`StaticMeshComponent.SetStaticMesh` (`self.Name Plate 301`) "/Game/Game/Art/Environments/Man-Made/Props/Furniture/NamePlate_302.NamePlate_302"))
    (:`NewEnumerator2`
      (`StaticMeshComponent.SetStaticMesh` (`self.Name Plate 301`) "/Game/Game/Art/Environments/Man-Made/Props/Furniture/NamePlate_303.NamePlate_303"))
    (:`NewEnumerator3`
      (`StaticMeshComponent.SetStaticMesh` (`self.Name Plate 301`) "/Game/Game/Art/Environments/Man-Made/Props/Furniture/NamePlate_304.NamePlate_304"))
    (:`NewEnumerator4`
      (`StaticMeshComponent.SetStaticMesh` (`self.Name Plate 301`) "/Game/Game/Art/Environments/Man-Made/Props/Furniture/NamePlate_305.NamePlate_305"))
    (:`NewEnumerator5`
      (`StaticMeshComponent.SetStaticMesh` (`self.Name Plate 301`) "/Game/Game/Art/Environments/Man-Made/Props/Furniture/NamePlate_306.NamePlate_306"))))