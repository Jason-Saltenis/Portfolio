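; BP_Keycard is an interactable keycard pickup that only the first-person character can collect.
; On interaction it registers the card with the character and plays a sound event.
; Through the player HUD, it flags key possession, overrides the madness bar value and prompts an optional image popup.
; It also calls LockDoor on an optional linked door, enables its close trigger, disables its open trigger, then destroys itself.
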(event `/Game/Jason/Interface/BPI_InteractInterface.InteractSuccess`
  (params (InteractingCaller :type "Actor Object Reference"))
  (bind _img (`self.Img`))
  (bind _closedoor (`self.closeDoor`))
  (bind _asbp_first_person_character (cast `/Game/FirstPerson/Blueprints/BP_FirstPersonCharacter` InteractingCaller))
  (`/Game/FirstPerson/Blueprints/BP_FirstPersonCharacter.PickupKeyCard` _asbp_first_person_character self)
  (`FMODBlueprintStatics.PlayEventAtLocation` "/Game/FMOD/Events/SFX/PopupKey.PopupKey" (`KismetMathLibrary.Conv_VectorToTransform` (`self.K2_GetActorLocation` self)))
  (bind _asplayer_hud (cast `PlayerHud` (`PlayerController.GetHUD` (`GameplayStatics.GetPlayerController` 0))))
  (bind _asbp_madness_bar (cast `/Game/Jason/UI/Blueprints/BP_MadnessBar` (`PlayerHud.CurrentWidget` _asplayer_hud)))
  (set `MyUserWidget.hasKey` true _asbp_madness_bar)
  (set `MyUserWidget.currentMadnessBarValue` 0.3 _asbp_madness_bar)
  (bind _aswbp_pop_up (cast `/Game/Haneul/Widget/WBP_PopUp` (`PlayerHud.PopUpWidget` _asplayer_hud)))
  (`/Engine/EditorBlueprintResources/StandardMacros.IsValid` _img
    (:`Is Valid`
      (`/Game/Haneul/Widget/WBP_PopUp.Prompt` _aswbp_pop_up _img false (0.769 1.4)))
    (:`Is Not Valid`
      _))
  (`/Engine/EditorBlueprintResources/StandardMacros.IsValid` _closedoor
    (:`Is Valid`
      (`/Game/Harnoorr/BP/BP_NEW/BP_TEST_DOOR.LockDoor` _closedoor "NewEnumerator0")
      (`PrimitiveComponent.SetCollisionEnabled` (`/Game/Harnoorr/BP/BP_NEW/BP_TEST_DOOR.CloseDoorTriggerbox` _closedoor) "QueryAndPhysics")
      (`PrimitiveComponent.SetCollisionEnabled` (`/Game/Harnoorr/BP/BP_NEW/BP_TEST_DOOR.OpenDoorTriggerbox` _closedoor) "NoCollision"))
    (:`Is Not Valid`
      _))
  (`self.K2_DestroyActor`))

(fn `CanInteract`
  (params (InteractingActor :type "Actor Object Reference"))
  (returns (CanInteract :type Boolean))
  (cast `/Game/FirstPerson/Blueprints/BP_FirstPersonCharacter` InteractingActor)
  (return true))

(fn `UserConstructionScript`)