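; Main menu wardrobe prop whose left door animates when the options menu is triggered.
; OptionsMenu alternates through a FlipFlop between playing a timeline that swings the left door and reversing it after a short delay.
; BeginPlay caches the 3D options widget actor, though nothing here uses it.
; PlayMenu is empty, leaving a double-door opening with a whoosh sound disconnected.
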(event `self.ReceiveBeginPlay`
  ; Begin Play
  (bind _returnvalue (`GameplayStatics.GetActorOfClass` "/Game/Jason/UI/Blueprints/Classes/BP_3D_Options_Widget.BP_3D_Options_Widget_C"))
  (set `self.3D Options Ref` _returnvalue))

(event `OptionsMenu`
  ; Options trigger
  (`/Engine/EditorBlueprintResources/StandardMacros.FlipFlop`
    (:`A`
      (bind (_direction _door_float_open) (`Timeline|Door Open/Close` :!label _label)
        (:`Update`
          (`SceneComponent.K2_SetRelativeRotation` (`self.Left_Door_Pivot`) (`KismetMathLibrary.MakeRotator` 0.0 0.0 (+ _door_float_open -10.0)) false false))))
    (:`B`
      (`KismetSystemLibrary.Delay` 1.0)
      (goto _label :!via `Reverse`))))

(event `Play Menu`
  ; Play Trigger
)

(fn `UserConstructionScript`)