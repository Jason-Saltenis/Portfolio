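; BP_TeleportDoor is an interactable portal door that swings open or closed on a timeline and toggles its linked TeleportTo door with it.
; Opening enables the trigger box, portal sound and, when linked, the portal plane.
; LoadLevel streams in the next loop level, teleports the player to an arrow and notifies the game mode.
; An optional tentacle part stays hidden until ShowElevatorPart spawns it, and an optional symbol sets the decal.
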(event `self.ReceiveBeginPlay`
  (bind _tentaclepart (`self.TentaclePart`))
  (bind _tentacle (`/Game/Haneul/Actor/BP_TentacleWallPart.Tentacle` _tentaclepart))
  (bind _rootcomponent (`Actor.RootComponent` _tentaclepart))
  (`PrimitiveComponent.SetCollisionEnabled` (`self.triggerBox`) "NoCollision")
  (`SceneComponent.SetVisibility` (`self.Plane`) false false)
  (`FMODAudioComponent.Stop` (`self.SFX_Portal`))
  (`KismetSystemLibrary.DelayUntilNextTick`)
  (`/Engine/EditorBlueprintResources/StandardMacros.IsValid` _tentaclepart
    (:`Is Valid`
      (`/Engine/EditorBlueprintResources/StandardMacros.IsValid` _rootcomponent
        (:`Is Valid`
          (`/Engine/EditorBlueprintResources/StandardMacros.IsValid` (`Actor.RootComponent` _tentacle)
            (:`Is Valid`
              (`SceneComponent.SetVisibility` _rootcomponent false true)
              (`SceneComponent.SetVisibility` (`Actor.RootComponent` _tentacle) false true)
              (`self.SetActorEnableCollision` _tentaclepart false)
              (`self.SetActorEnableCollision` _tentacle false)
              (`TentacleWall.StartDown` _tentaclepart)
              (`FMODAudioComponent.Stop` (`/Game/Harnoorr/BP/BP_NEW/BP_TENTACLE_part.SFX_Tenticle` _tentacle)))))))))

(event `/Game/Jason/Interface/BPI_InteractInterface.InteractSuccess`
  (params (InteractingCaller :type "Actor Object Reference"))
  (bind _sfx_portal (`self.SFX_Portal`))
  (bind _teleportto (`self.teleportTo`))
  (cast `/Game/Haneul/Actor/BP_TeleportDoor` InteractingCaller
    (:`then`
      _)
    (:`CastFailed`
      (`/Engine/EditorBlueprintResources/StandardMacros.IsValid` _teleportto
        (:`Is Valid`
          (bind _asbp_teleport_door (cast `/Game/Haneul/Actor/BP_TeleportDoor` _teleportto))
          (`self.InteractSuccess` _asbp_teleport_door self))
        (:`Is Not Valid`
          _))))
  (switch `/Game/Jason/Enums/En_DoorStatus` (`self.Status`)
    (:`NewEnumerator0`
      (`FMODAudioComponent.Play` _sfx_portal)
      (`self.OpenCloseDoor` true)
      (bind (_direction _door_float) (`Timeline|Timeline` :!label _label)
        (:`Update`
          (`SceneComponent.K2_SetRelativeRotation` (`self.DoorScene`) (`KismetMathLibrary.MakeRotator` 0.0 0.0 _door_float) false false))
        (:`Finished`
          (`PrimitiveComponent.SetCollisionEnabled` (`self.DoorMesh`) "QueryAndPhysics"))))
    (:`NewEnumerator1`
      (`FMODAudioComponent.Stop` _sfx_portal)
      (`self.OpenCloseDoor` false)
      (goto _label :!via `Reverse`))))

(event `self.ShowElevatorPart`
  (bind _tentaclepart (`self.TentaclePart`))
  (`FMODBlueprintStatics.PlayEvent2D` "/Game/FMOD/Events/SFX/Teleport.Teleport")
  (`/Engine/EditorBlueprintResources/StandardMacros.IsValid` _tentaclepart
    (:`Is Valid`
      (`SceneComponent.SetVisibility` (`Actor.RootComponent` _tentaclepart) true true)
      (`SceneComponent.SetVisibility` (`Actor.RootComponent` (`/Game/Haneul/Actor/BP_TentacleWallPart.Tentacle` _tentaclepart)) true true)
      (`self.SetActorEnableCollision` _tentaclepart true)
      (`self.SetActorEnableCollision` (`/Game/Haneul/Actor/BP_TentacleWallPart.Tentacle` _tentaclepart) true)
      (`TentacleWall.Spawn` _tentaclepart)
      (`FMODAudioComponent.Play` (`/Game/Harnoorr/BP/BP_NEW/BP_TENTACLE_part.SFX_Tenticle` (`/Game/Haneul/Actor/BP_TentacleWallPart.Tentacle` _tentaclepart))))))

(event `/Game/Jason/Interface/BPI_InteractInterface.InteractFail`
  (params (`Interacting Actor` :type "Actor Object Reference"))
  (`FMODBlueprintStatics.PlayEventAtLocation` "/Game/FMOD/Events/SFX/DoorLock.DoorLock" (`KismetMathLibrary.Conv_VectorToTransform` (`self.K2_GetActorLocation` self))))

(event `self.LoadLevel`
  (`/Engine/EditorBlueprintResources/StandardMacros.IsValid` (`self.nextLevelArrow`)
    (:`Is Valid`
      (`GameplayStatics.LoadStreamLevelBySoftObjectPtr` (`self.NextLoopLevel`) true true)
      (`self.Teleport` (`Controller.K2_GetPawn` (`GameplayStatics.GetPlayerController` 0)) (`self.nextLevelArrow`))
      (bind _assweet_spot_game_mode (cast `SweetSpotGameMode` (`GameplayStatics.GetGameMode`)))
      (`SweetSpotGameMode.CheckForSubLevel` _assweet_spot_game_mode (`self.thisLoopLevel`)))))

(fn `CanInteract`
  (params (InteractingActor :type "Actor Object Reference"))
  (returns (CanInteract :type Boolean))
  (cast `/Game/FirstPerson/Blueprints/BP_FirstPersonCharacter` InteractingActor)
  (return true))

(fn `OpenCloseDoor`
  (params (OpenDoor :type Boolean))
  (bind _triggerbox (`self.triggerBox`))
  (if OpenDoor
    (set `self.Status` "NewEnumerator1")
    (`FMODBlueprintStatics.PlayEvent2D` "/Game/FMOD/Events/Foley/OpenDoor.OpenDoor")
    (`PrimitiveComponent.SetCollisionEnabled` _triggerbox "QueryAndPhysics")
    (else
      (set `self.Status` "NewEnumerator0")
      (`FMODBlueprintStatics.PlayEvent2D` "/Game/FMOD/Events/SFX/DoorClose.DoorClose")
      (`PrimitiveComponent.SetCollisionEnabled` _triggerbox "NoCollision")))
  (`FMODBlueprintStatics.PlayEvent2D` null)
  (`PrimitiveComponent.SetCollisionEnabled` (`self.DoorMesh`) "NoCollision")
  (`/Engine/EditorBlueprintResources/StandardMacros.IsValid` (`self.teleportTo`)
    (:`Is Valid`
      (`SceneComponent.SetVisibility` (`self.Plane`) OpenDoor false))))

(fn `UserConstructionScript`
  (bind _decal (`self.Decal`))
  (bind _symbol (`self.Symbol`))
  (`/Engine/EditorBlueprintResources/StandardMacros.IsValid` _symbol
    (:`Is Valid`
      (`DecalComponent.SetDecalMaterial` _decal _symbol))
    (:`Is Not Valid`
      (`ActorComponent.K2_DestroyComponent` _decal))))