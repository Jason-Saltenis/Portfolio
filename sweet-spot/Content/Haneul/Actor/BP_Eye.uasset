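; BP_Eye is an eye actor, built from eye, iris and eyelid meshes, that can close and reopen through animation.
; BeginPlay sets the custom depth stencil value of the meshes to zero.
; CloseEye plays one-shot animations on the eye and both lids, then CustomEvent waits briefly, snaps their playback position and pauses them.
; OpenEye unpauses those animations so they continue from the held pose.
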(event `self.ReceiveBeginPlay`
  (`PrimitiveComponent.SetCustomDepthStencilValue` (`self.EyelidHigher_low`) 0)
  (`PrimitiveComponent.SetCustomDepthStencilValue` (`self.Iris_low`) 0)
  (`PrimitiveComponent.SetCustomDepthStencilValue` (`self.EyelidLower_low`) 0)
  (`PrimitiveComponent.SetCustomDepthStencilValue` (`self.Eye`) 0))

(event `CustomEvent`
  (bind _eye (`self.Eye`))
  (`KismetSystemLibrary.Delay` 0.2)
  (`SkeletalMeshComponent.SetPosition` _eye 0.2 true)
  (`SkeletalMeshComponent.SetPosition` (`self.EyelidLower_low`) 0.2 true)
  (`SkeletalMeshComponent.SetPosition` (`self.EyelidHigher_low`) 0.2 true)
  (set `SkeletalMeshComponent.bPauseAnims` true _eye)
  (set `SkeletalMeshComponent.bPauseAnims` true (`self.EyelidHigher_low`))
  (set `SkeletalMeshComponent.bPauseAnims` true (`self.EyelidLower_low`)))

(fn `CloseEye`
  (`SkeletalMeshComponent.PlayAnimation` (`self.Eye`) null false)
  (`SkeletalMeshComponent.PlayAnimation` (`self.EyelidLower_low`) null false)
  (`SkeletalMeshComponent.PlayAnimation` (`self.EyelidHigher_low`) null false)
  (`self.CustomEvent`))

(fn `OpenEye`
  (set `SkeletalMeshComponent.bPauseAnims` false (`self.Eye`))
  (set `SkeletalMeshComponent.bPauseAnims` false (`self.EyelidHigher_low`))
  (set `SkeletalMeshComponent.bPauseAnims` false (`self.EyelidLower_low`)))

(fn `UserConstructionScript`)