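; BP_Smoke is a smoke sphere actor whose size responds to the player's madness meter.
; On BeginPlay it grabs the first top-level MyUserWidget as the madness meter reference.
; Each Tick it reads the clamped madness bar value and scales the smoke sphere larger when that value falls within its Min–Max range, smaller otherwise.
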(event `self.ReceiveBeginPlay`
  (bind _foundwidgets (`WidgetBlueprintLibrary.GetAllWidgetsOfClass` "/Script/UnrealProjectBase.MyUserWidget"))
  (set `self.HanMadnessMeter` (`|GetArrayItem` _foundwidgets)))

(event `self.ReceiveTick`
  (params (DeltaSeconds :type "Float (single-precision)"))
  (bind _smoke_sphere (`self.Smoke_Sphere`))
  (`/Engine/EditorBlueprintResources/StandardMacros.IsValid` (`self.HanMadnessMeter`)
    (:`Is Valid`
      (if (`KismetMathLibrary.InRange_FloatFloat` (`KismetMathLibrary.FClamp` (`MyUserWidget.mmadnessBarValue` (`self.HanMadnessMeter`))) (`self.Min`) (`self.Max`))
        (bind _output_get (set `self.SphereSize` (10.0 10.0 10.0)))
        (`SceneComponent.SetRelativeScale3D` _smoke_sphere _output_get)
        (else
          (bind _output_get_2 (set `self.SphereSize` (7.0 7.0 7.0)))
          (`SceneComponent.SetRelativeScale3D` _smoke_sphere _output_get_2))))))

(fn `UserConstructionScript`)