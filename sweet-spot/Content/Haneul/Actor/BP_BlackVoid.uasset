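; BP_BlackVoid is a tentacled, eyed void hazard that sends the player to another level on contact.
; On BeginPlay it spawns a hidden tentacle at each arrow component, hides the eyes and disables its Box collision.
; PlaySound reveals them, plays the void sound and enables Box.
; Player capsule overlap with TriggerBox or Box swaps sublevels through SweetSpotGameMode and zeroes the HUD madness meter.
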(event `self.ReceiveBeginPlay`
  (`FMODAudioComponent.Stop` (`self.BlackVoid_SFX`))
  (for _array_element (`self.K2_GetComponentsByClass` "/Script/Engine.ArrowComponent")
    (bind _returnvalue (`|SpawnActorFromClass` "/Game/Harnoorr/BP/BP_NEW/BP_TENTACLE.BP_TENTACLE_C" (`SceneComponent.K2_GetComponentToWorld` _array_element) "AlwaysSpawn" "MultiplyWithRoot" null null))
    (`KismetArrayLibrary.Array_Add` (`self.tentacle`) _returnvalue)
    (`self.K2_AttachToComponent` _returnvalue (`self.Arrow`) "None" "KeepWorld" "KeepWorld" "KeepWorld" true)
    (`PrimitiveComponent.SetCollisionEnabled` (`/Game/Harnoorr/BP/BP_NEW/BP_TENTACLE.Box` _returnvalue) "NoCollision")
    (`self.SetActorHiddenInGame` _returnvalue true))
  (`SceneComponent.SetHiddenInGame` (`self.eyeGroup`) true true)
  (`PrimitiveComponent.SetCollisionEnabled` (`self.Box`) "NoCollision"))

(event `self.triggerBox.OnComponentBeginOverlap`
  (params (OverlappedComponent :type "PrimitiveComponent Object Reference") (OtherActor :type "Actor Object Reference") (OtherComp :type "PrimitiveComponent Object Reference") (OtherBodyIndex :type Integer) (bFromSweep :type Boolean) (SweepResult :type "HitResult Structure (by ref)"))
  (cast `/Game/FirstPerson/Blueprints/BP_FirstPersonCharacter` OtherActor)
  (cast `CapsuleComponent` OtherComp)
  (bind _assweet_spot_game_mode (cast `SweetSpotGameMode` (`GameplayStatics.GetGameMode`) :!label _label))
  (`SweetSpotGameMode.UnloadThenLoadLevel` _assweet_spot_game_mode (`self.CurrentLevel`) (`self.levelToLoad`))
  (bind _asplayer_hud (cast `PlayerHud` (`PlayerController.GetHUD` (`GameplayStatics.GetPlayerController` 0))))
  (set `MyUserWidget.currentMadnessBarValue` 0.0 (`PlayerHud.GetMadnessMeterWidget` _asplayer_hud)))

(event `self.Box.OnComponentBeginOverlap`
  (params (OverlappedComponent :type "PrimitiveComponent Object Reference") (OtherActor :type "Actor Object Reference") (OtherComp :type "PrimitiveComponent Object Reference") (OtherBodyIndex :type Integer) (bFromSweep :type Boolean) (SweepResult :type "HitResult Structure (by ref)"))
  (cast `/Game/FirstPerson/Blueprints/BP_FirstPersonCharacter` OtherActor)
  (cast `CapsuleComponent` OtherComp)
  (goto _label))

(event `self.PlaySound`
  (`FMODAudioComponent.Play` (`self.BlackVoid_SFX`))
  (for _array_element (`self.tentacle`)
    (`self.SetActorHiddenInGame` _array_element false)
    (`SceneComponent.SetHiddenInGame` (`self.EyeRoot`) false true))
  (`SceneComponent.SetHiddenInGame` (`self.eyeGroup`) false true)
  (`PrimitiveComponent.SetCollisionEnabled` (`self.Box`) "QueryAndPhysics"))

(event `self.ReceiveEndPlay`
  (params (EndPlayReason :type "EEndPlayReason Enum" :default "Destroyed"))
  (for _array_element (`self.tentacle`)
    (`self.K2_DestroyActor` _array_element)))

(fn `UserConstructionScript`)