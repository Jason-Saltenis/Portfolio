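; BP_Static is an actor that sets the scale of its StaticShape component from a madness meter's bar value.
; Each Tick, if the MadnessMeter reference is valid, it clamps the value to 0–1 and range-checks it, switching between a larger and a smaller uniform scale.
; The construction script and NewFunction are empty.
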(event `self.ReceiveTick`
  (params (DeltaSeconds :type "Float (single-precision)"))
  (bind _static_shape (`self.Static Shape`))
  (`/Engine/EditorBlueprintResources/StandardMacros.IsValid` (`self.MadnessMeter`)
    (:`Is Valid`
      (if (`KismetMathLibrary.InRange_FloatFloat` (`KismetMathLibrary.FClamp` (`MyUserWidget.mmadnessBarValue` (`self.MadnessMeter`))))
        (bind _output_get (set `self.ShapeSize` (10.0 10.0 10.0)))
        (`SceneComponent.SetRelativeScale3D` _static_shape _output_get)
        (else
          (bind _output_get_2 (set `self.ShapeSize` (7.0 7.0 7.0)))
          (`SceneComponent.SetRelativeScale3D` _static_shape _output_get_2))))))

(fn `NewFunction`)

(fn `UserConstructionScript`)