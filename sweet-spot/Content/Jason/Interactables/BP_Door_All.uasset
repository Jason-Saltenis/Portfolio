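; Interactable door that swings open and closed, restricted to players with a matching keycard color or a SweetSpot.Unlocked gameplay tag.
; CanInteract checks the interacting first-person character's tag and keycard color against DoorColor.
; Successful interaction toggles Status, plays a sound event and plays or reverses a timeline driving DoorScene yaw, while failure plays a sound at the door.
; KeycardCheck is an empty stub with leftover unconnected debug logic.
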(event `/Game/Jason/Interface/BPI_InteractInterface.InteractSuccess`
  (params (InteractingCaller :type "Actor Object Reference"))
  (switch `/Game/Jason/Enums/En_DoorStatus` (`self.Status`)
    (:`NewEnumerator0`
      (`KismetSystemLibrary.PrintString` "Open")
      (`FMODBlueprintStatics.PlayEvent2D` null)
      (set `self.Status` "NewEnumerator1")
      (bind (_direction _door_float) (`Timeline|OpenDoor_Timeline` :!label _label)
        (:`Update`
          (`SceneComponent.K2_SetRelativeRotation` (`self.DoorScene`) (`KismetMathLibrary.MakeRotator` 0.0 0.0 _door_float) false false))))
    (:`NewEnumerator1`
      (`KismetSystemLibrary.PrintString` "Close")
      (`FMODBlueprintStatics.PlayEvent2D` null)
      (set `self.Status` "NewEnumerator0")
      (goto _label :!via `Reverse`))))

(event `/Game/Jason/Interface/BPI_InteractInterface.InteractFail`
  (params (`Interacting Actor` :type "Actor Object Reference"))
  (`FMODBlueprintStatics.PlayEventAtLocation` null (`KismetMathLibrary.Conv_VectorToTransform` (`self.K2_GetActorLocation` self))))

(fn `CanInteract`
  (params (InteractingActor :type "Actor Object Reference"))
  (returns (CanInteract :type Boolean))
  (bind _asbp_first_person_character (cast `/Game/FirstPerson/Blueprints/BP_FirstPersonCharacter` InteractingActor))
  (bind _returnvalue (message `GameplayTagAssetInterface.HasAnyMatchingGameplayTags` InteractingActor (`BlueprintGameplayTagLibrary.MakeGameplayTagContainerFromArray` (`|MakeArray` (struct :`TagName` "SweetSpot.Unlocked") :!type "GameplayTag Structure"))))
  (return (or _returnvalue (== (`/Game/FirstPerson/Blueprints/BP_FirstPersonCharacter.KeycardColor` _asbp_first_person_character) (`self.DoorColor`)))))

(fn `Keycard_Check`)

(fn `UserConstructionScript`)