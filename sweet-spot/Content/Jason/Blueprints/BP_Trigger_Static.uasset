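; BP_Trigger_Static is a trigger box that toggles a BP_Static actor on whatever actor overlaps it.
; Entering spawns BP_Static attached to that actor, or detaches and destroys it if the stored reference is still valid.
; A DoOnce, reset on end overlap, limits this to one toggle per entry.
; An unconnected branch would cast to BP_FirstPersonCharacter and destroy an actor when the madness meter is full.
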(event `self.Box.OnComponentBeginOverlap`
  (params (OverlappedComponent :type "PrimitiveComponent Object Reference") (OtherActor :type "Actor Object Reference") (OtherComp :type "PrimitiveComponent Object Reference") (OtherBodyIndex :type Integer) (bFromSweep :type Boolean) (SweepResult :type "HitResult Structure (by ref)"))
  (bind _bp_static_ref (`self.BP_Static_ref`))
  (`/Engine/EditorBlueprintResources/StandardMacros.DoOnce` false :!label _label
    (:`Completed`
      (if (`KismetSystemLibrary.IsValid` _bp_static_ref)
        (`self.K2_DetachFromActor` _bp_static_ref "KeepRelative" "KeepRelative" "KeepRelative")
        (`self.K2_DestroyActor` _bp_static_ref)
        (else
          (bind _returnvalue (`|SpawnActorFromClass` "/Game/Jason/Blueprints/BP_Static.BP_Static_C" (`self.GetTransform` OtherActor) "AlwaysSpawn" "MultiplyWithRoot" null null))
          (bind _output_get (set `self.BP_Static_ref` _returnvalue))
          (`self.K2_AttachToActor` _output_get OtherActor "None" "SnapToTarget" "KeepRelative" "KeepRelative" true))))))

(event `self.Box.OnComponentEndOverlap`
  (params (OverlappedComponent :type "PrimitiveComponent Object Reference") (OtherActor :type "Actor Object Reference") (OtherComp :type "PrimitiveComponent Object Reference") (OtherBodyIndex :type Integer))
  (goto _label :!via `Reset`))

(fn `UserConstructionScript`)