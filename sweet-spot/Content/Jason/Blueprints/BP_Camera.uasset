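; BP_Camera is a menu camera that moves between placed Camera_Position actors, starting at the main menu view.
; On BeginPlay it shows the mouse cursor, sets game-and-UI input and snaps to the actor tagged OriginalMainMenuCam.
; ChangeCam records the current transform, then uses the CamerSwitch timeline to lerp to the transform of CurrentCam, which is not assigned in this graph.
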(event `self.ReceiveBeginPlay`
  (bind _returnvalue (`GameplayStatics.GetPlayerController` 0))
  (set `PlayerController.bShowMouseCursor` true _returnvalue)
  (`WidgetBlueprintLibrary.SetInputMode_GameAndUIEx` _returnvalue null "DoNotLock" false)
  (bind _outactors (`GameplayStatics.GetAllActorsWithTag` "OriginalMainMenuCam"))
  (bind _ascamera_position (cast `/Game/Jason/Blueprints/Camera_Position` (`|GetArrayItem` _outactors)))
  (`self.K2_SetActorTransform` (`self.GetTransform` _ascamera_position)))

(event `ChangeCam`
  (set `self.CurrentPosition` (`self.GetTransform`))
  (bind (_direction _camera_value_position) (`Timeline|CamerSwitch` :!via `PlayFromStart`)
    (:`Update`
      (`self.K2_SetActorTransform` (`KismetMathLibrary.TLerp` (`self.CurrentPosition`) (`self.GetTransform` (`self.CurrentCam`)) _camera_value_position)))))

(fn `UserConstructionScript`)