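; Interactable door that swings open and closed, gated by a match between its DoorColor and the first-person character's KeycardColor.
; A successful interaction flips Status and plays or reverses a timeline driving DoorScene's yaw; failure plays an FMOD sound.
; Two overlap colliders, one marked temporary for closing, also trigger the toggle through DoOnce gates without checking the keycard.
; KeycardCheck holds only disconnected leftover logic.
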(event `self.Box.OnComponentBeginOverlap`
  (params (OverlappedComponent :type "PrimitiveComponent Object Reference") (OtherActor :type "Actor Object Reference") (OtherComp :type "PrimitiveComponent Object Reference") (OtherBodyIndex :type Integer) (bFromSweep :type Boolean) (SweepResult :type "HitResult Structure (by ref)"))
  (`/Engine/EditorBlueprintResources/StandardMacros.DoOnce` false :!label _label
    (:`Completed`
      (switch `/Game/Jason/Enums/En_DoorStatus` (`self.Status`) :!label _label_2
        (:`NewEnumerator0`
          (set `self.Status` "NewEnumerator1")
          (bind (_direction _door_float) (`Timeline|OpenDoor_Timeline` :!label _label_3)
            (:`Update`
              (`SceneComponent.K2_SetRelativeRotation` (`self.DoorScene`) (`KismetMathLibrary.MakeRotator` 0.0 0.0 _door_float) false false))))
        (:`NewEnumerator1`
          (set `self.Status` "NewEnumerator0")
          (`|ExecutionSequence`
            (:`then_0`
              (goto _label_3 :!via `Reverse`))
            (:`then_1`
              (goto _label :!via `Reset`))))))))

(event `self.InteractSuccess`
  (params (InteractingCaller :type "Actor Object Reference"))
  (goto _label_2))

(event `self.TEMP COLLIDER TO CLOSE DOOR.OnComponentBeginOverlap`
  (params (OverlappedComponent :type "PrimitiveComponent Object Reference") (OtherActor :type "Actor Object Reference") (OtherComp :type "PrimitiveComponent Object Reference") (OtherBodyIndex :type Integer) (bFromSweep :type Boolean) (SweepResult :type "HitResult Structure (by ref)"))
  (if true
    (`/Engine/EditorBlueprintResources/StandardMacros.DoOnce` false :!label _label_4
      (:`Completed`
        (goto _label_2)))
    (else
      (goto _label_4 :!via `Reset`))))

(event `self.InteractFail`
  (params (`Interacting Actor` :type "Actor Object Reference"))
  (`FMODBlueprintStatics.PlayEventAtLocation` "/Game/FMOD/Events/SFX/MattressCollisionEnter.MattressCollisionEnter" (`KismetMathLibrary.Conv_VectorToTransform` (`self.K2_GetActorLocation` self))))

(fn `CanInteract`
  (params (InteractingActor :type "Actor Object Reference"))
  (returns (CanInteract :type Boolean))
  (bind _asbp_first_person_character (cast `/Game/FirstPerson/Blueprints/BP_FirstPersonCharacter` InteractingActor))
  (return (== (`/Game/FirstPerson/Blueprints/BP_FirstPersonCharacter.KeycardColor` _asbp_first_person_character) (`self.DoorColor`))))

(fn `Keycard_Check`)

(fn `UserConstructionScript`)