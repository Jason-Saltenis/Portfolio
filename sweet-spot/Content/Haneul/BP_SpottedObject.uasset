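; BP_SpottedObject is a component for BP_Eye that reacts to fade, reset and look-at events.
; FadeAway, gated by IsClosingAnim, closes the eye, sets custom depth stencil on its skeletal meshes and starts a focus camera shake.
; ResetPosition reopens the eye, clears the stencil and stops all camera shakes.
; LookatPlayer rotates the eye root to face the first-person camera.
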(event `self.FadeAway`
  (if (not (`self.isClosingAnim`))
    (bind _asbp_eye (cast `/Game/Haneul/Actor/BP_Eye` (`self.GetOwner`)))
    (`/Game/Haneul/Actor/BP_Eye.CloseEye` _asbp_eye)
    (for _array_element (`Actor.K2_GetComponentsByClass` _asbp_eye "/Script/Engine.SkeletalMeshComponent")
      (`PrimitiveComponent.SetCustomDepthStencilValue` _array_element 1))
    (`PlayerCameraManager.StartCameraShake` :`self` (`GameplayStatics.GetPlayerCameraManager` 0) :`ShakeClass` "/Game/Haneul/CameraShake/BP_CamShakeFocus.BP_CamShakeFocus_C")))

(event `self.ResetPosition`
  (bind _asbp_eye (cast `/Game/Haneul/Actor/BP_Eye` (`self.GetOwner`)))
  (`/Game/Haneul/Actor/BP_Eye.OpenEye` _asbp_eye)
  (for _array_element (`Actor.K2_GetComponentsByClass` _asbp_eye "/Script/Engine.SkeletalMeshComponent")
    (`PrimitiveComponent.SetCustomDepthStencilValue` _array_element 0))
  (`PlayerCameraManager.StopAllCameraShakes` (`GameplayStatics.GetPlayerCameraManager` 0) true))

(event `self.LookAtPlayer`
  (bind _asbp_eye (cast `/Game/Haneul/Actor/BP_Eye` (`self.GetOwner`)))
  (bind _asbp_first_person_character (cast `/Game/FirstPerson/Blueprints/BP_FirstPersonCharacter` (`Controller.K2_GetPawn` (`GameplayStatics.GetPlayerController` 0))))
  (bind _eyeroot (`/Game/Haneul/Actor/BP_Eye.EyeRoot` _asbp_eye))
  (`SceneComponent.K2_SetWorldRotation` _eyeroot (`KismetMathLibrary.FindLookAtRotation` (`SceneComponent.K2_GetComponentLocation` _eyeroot) (`SceneComponent.K2_GetComponentLocation` (`/Game/FirstPerson/Blueprints/BP_FirstPersonCharacter.FirstPersonCamera` _asbp_first_person_character))) false false))