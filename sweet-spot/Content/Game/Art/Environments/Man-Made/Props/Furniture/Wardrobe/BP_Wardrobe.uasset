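; BP_Wardrobe is an interactable wardrobe prop whose two doors the first-person player character can open and close.
; A successful interaction plays a wood creak sound and uses a FlipFlop to play or reverse a timeline that yaws the door pivots in opposite directions.
; Door collision is disabled on interaction and restored when the timeline finishes.
; CanInteract only accepts BP_FirstPersonCharacter as the interacting actor.
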(event `/Game/Jason/Interface/BPI_InteractInterface.InteractSuccess`
  (params (InteractingCaller :type "Actor Object Reference"))
  (`PrimitiveComponent.SetCollisionEnabled` (`self.Wardrobe_Door01`) "NoCollision")
  (`PrimitiveComponent.SetCollisionEnabled` (`self.Wardrobe_Door02`) "NoCollision")
  (`FMODBlueprintStatics.PlayEventAtLocation` "/Game/FMOD/Events/SFX/WoodCreak.WoodCreak" (`self.Location`))
  (`/Engine/EditorBlueprintResources/StandardMacros.FlipFlop`
    (:`A`
      (bind (_direction _rotate_door) (`Timeline|Timeline` :!label _label)
        (:`Update`
          (`SceneComponent.K2_SetRelativeRotation` (`self.RightDoorPivot`) (`KismetMathLibrary.MakeRotator` 0.0 0.0 (* _rotate_door -1.0)) false false)
          (`SceneComponent.K2_SetRelativeRotation` (`self.LeftDoorPivot`) (`KismetMathLibrary.MakeRotator` 0.0 0.0 _rotate_door) false false))
        (:`Finished`
          (`PrimitiveComponent.SetCollisionEnabled` (`self.Wardrobe_Door01`) "QueryAndPhysics")
          (`PrimitiveComponent.SetCollisionEnabled` (`self.Wardrobe_Door02`) "QueryAndPhysics"))))
    (:`B`
      (goto _label :!via `Reverse`))))

(fn `CanInteract`
  (params (InteractingActor :type "Actor Object Reference"))
  (returns (CanInteract :type Boolean))
  (cast `/Game/FirstPerson/Blueprints/BP_FirstPersonCharacter` InteractingActor)
  (return true))

(fn `UserConstructionScript`)