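; BP_NormalRemote is an interactable remote that only the first-person character can use.
; A successful interaction shakes the camera at the player and raises the HUD madness bar by a fixed step.
; A pickup event destroys the remote, BP_Smoke and BP_TriggerSmoke, but the nodes binding it to the character are disconnected from the empty overlap events.
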(event `/Game/Jason/Interface/BPI_InteractInterface.InteractSuccess`
  (params (InteractingCaller :type "Actor Object Reference"))
  (`self.CameraShake`)
  (`self.IncreaseMadness`))

(event `self.ReceiveActorBeginOverlap`
  (params (OtherActor :type "Actor Object Reference")))

(event `Remote_Pickup_Event`
  (bind _returnvalue (`GameplayStatics.GetActorOfClass` "/Game/Jason/Blueprints/BP_Smoke.BP_Smoke_C"))
  (bind _returnvalue_2 (`GameplayStatics.GetActorOfClass` "/Game/Jason/Blueprints/BP_TriggerSmoke.BP_TriggerSmoke_C"))
  (`self.K2_DestroyActor` self)
  (`self.K2_DestroyActor` _returnvalue)
  (`self.K2_DestroyActor` _returnvalue_2))

(event `self.ReceiveActorEndOverlap`
  (params (OtherActor :type "Actor Object Reference")))

(fn `CameraShake`
  (`GameplayStatics.PlayWorldCameraShake` "/Game/Haneul/BP_CamShakeMenu.BP_CamShakeMenu_C" (`self.K2_GetActorLocation` (`Controller.K2_GetPawn` (`GameplayStatics.GetPlayerController` 0))) 0.0 500.0))

(fn `CanInteract`
  (params (InteractingActor :type "Actor Object Reference"))
  (returns (CanInteract :type Boolean))
  (cast `/Game/FirstPerson/Blueprints/BP_FirstPersonCharacter` InteractingActor)
  (return true))

(fn `IncreaseMadness`
  (bind _asplayer_controller (cast `PlayerController` (`GameplayStatics.GetPlayerController` 0)))
  (bind _asplayer_hud (cast `PlayerHud` (`PlayerController.GetHUD` _asplayer_controller)))
  (bind _asbp_madness_bar (cast `/Game/Jason/UI/Blueprints/BP_MadnessBar` (`PlayerHud.GetMadnessMeterWidget` _asplayer_hud)))
  (`MyUserWidget.IncreaseMadnessBar` _asbp_madness_bar 0.2))

(fn `UserConstructionScript`)