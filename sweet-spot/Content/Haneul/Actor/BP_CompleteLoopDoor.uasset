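; BP_CompleteLoopDoor is a doorway actor that marks a teleport loop as completed when a character passes through it.
; Two overlap triggers fire in sequence: Box arms EndOverlap, which starts with collision disabled, and both accept only a Character's capsule.
; EndOverlap sets IsCompleted on the referenced Teleport, then, if Exit is valid, turns on its light and enables the initially non-colliding Wall.
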(event `self.ReceiveBeginPlay`
  (`PrimitiveComponent.SetCollisionEnabled` (`self.Box`) "QueryAndPhysics")
  (`PrimitiveComponent.SetCollisionEnabled` (`self.Wall`) "NoCollision"))

(event `self.Box.OnComponentBeginOverlap`
  (params (OverlappedComponent :type "PrimitiveComponent Object Reference") (OtherActor :type "Actor Object Reference") (OtherComp :type "PrimitiveComponent Object Reference") (OtherBodyIndex :type Integer) (bFromSweep :type Boolean) (SweepResult :type "HitResult Structure (by ref)"))
  (cast `Character` OtherActor)
  (cast `CapsuleComponent` OtherComp)
  (`PrimitiveComponent.SetCollisionEnabled` (`self.endOverlap`) "QueryAndPhysics"))

(event `self.endOverlap.OnComponentBeginOverlap`
  (params (OverlappedComponent :type "PrimitiveComponent Object Reference") (OtherActor :type "Actor Object Reference") (OtherComp :type "PrimitiveComponent Object Reference") (OtherBodyIndex :type Integer) (bFromSweep :type Boolean) (SweepResult :type "HitResult Structure (by ref)"))
  (bind _teleport (`self.Teleport`))
  (bind _exit (`self.Exit`))
  (cast `Character` OtherActor)
  (cast `CapsuleComponent` OtherComp)
  (`/Engine/EditorBlueprintResources/StandardMacros.IsValid` _teleport
    (:`Is Valid`
      (set `MyTeleport.isCompleted` true _teleport))
    (:`Is Not Valid`
      _))
  (`/Engine/EditorBlueprintResources/StandardMacros.IsValid` _exit
    (:`Is Valid`
      (`/Game/Harnoorr/BP/BP_EXIT.TurnLightOn` _exit)
      (`PrimitiveComponent.SetCollisionEnabled` (`self.Wall`) "QueryAndPhysics"))))

(fn `UserConstructionScript`
  (`PrimitiveComponent.SetCollisionEnabled` (`self.endOverlap`) "NoCollision")
  (`PrimitiveComponent.SetCollisionEnabled` (`self.Box`) "QueryAndPhysics"))