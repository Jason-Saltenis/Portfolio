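; BP_ExitDoor_Loop0 is an interactable exit door that swings open or closed with sound, optionally requiring a keycard matching its color.
; A successful interaction toggles it along with any linked Door, using a Timeline for yaw and disabling collision during the swing.
; An optional trigger box, sized in the construction script, closes an open door when the player's capsule overlaps it.
; An AddPortal flag reveals its Plane at BeginPlay.
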(event `self.ReceiveBeginPlay`
  (if (`self.AddPortal`)
    (`SceneComponent.SetVisibility` (`self.Plane`) true false)))

(event `ConnectDoor`
  (`PrimitiveComponent.SetCollisionEnabled` (`self.ExitDoor`) "NoCollision" :!label _label)
  (switch `/Game/Jason/Enums/En_DoorStatus` (`self.DoorStatus`)
    (:`NewEnumerator0`
      (`FMODBlueprintStatics.PlayEventAtLocation` "/Game/FMOD/Events/Door/Door_Open_Creak.Door_Open_Creak" (`KismetMathLibrary.Conv_VectorToTransform` (`self.K2_GetActorLocation` self)))
      (set `self.DoorStatus` "NewEnumerator1")
      (bind (_direction _door_float) (`Timeline|Timeline` :!label _label_2)
        (:`Update`
          (`SceneComponent.K2_SetRelativeRotation` (`self.ExitDoor`) (`KismetMathLibrary.MakeRotator` 0.0 0.0 _door_float) false false))
        (:`Finished`
          (`PrimitiveComponent.SetCollisionEnabled` (`self.ExitDoor`) "QueryAndPhysics"))))
    (:`NewEnumerator1`
      (`FMODBlueprintStatics.PlayEventAtLocation` "/Game/FMOD/Events/Door/Door_Wood_Close.Door_Wood_Close" (`KismetMathLibrary.Conv_VectorToTransform` (`self.K2_GetActorLocation` self)))
      (set `self.DoorStatus` "NewEnumerator0")
      (goto _label_2 :!via `Reverse`))))

(event `self.InteractSuccess`
  (params (InteractingCaller :type "Actor Object Reference"))
  (bind _door (`self.Door`))
  (`/Engine/EditorBlueprintResources/StandardMacros.IsValid` _door
    (:`Is Valid`
      (`self.ConnectDoor` _door)
      (goto _label))
    (:`Is Not Valid`
      (goto _label))))

(event `self.InteractFail`
  (params (`Interacting Actor` :type "Actor Object Reference")))

(event `self.Box.OnComponentBeginOverlap`
  (params (OverlappedComponent :type "PrimitiveComponent Object Reference") (OtherActor :type "Actor Object Reference") (OtherComp :type "PrimitiveComponent Object Reference") (OtherBodyIndex :type Integer) (bFromSweep :type Boolean) (SweepResult :type "HitResult Structure (by ref)"))
  (cast `/Game/FirstPerson/Blueprints/BP_FirstPersonCharacter` OtherActor)
  (cast `CapsuleComponent` OtherComp)
  (if (not (`|EnumEquality` (`self.DoorStatus`) "NewEnumerator0"))
    (`/Game/Jason/Interface/BPI_InteractInterface.InteractSuccess` null)))

(fn `CanInteract`
  (params (InteractingActor :type "Actor Object Reference"))
  (returns (CanInteract :type Boolean))
  (bind _doorcolor (`self.DoorColor`))
  (bind _asbp_first_person_character (cast `/Game/FirstPerson/Blueprints/BP_FirstPersonCharacter` InteractingActor))
  (if (== _doorcolor (struct))
    _
    (elif (== (`/Game/FirstPerson/Blueprints/BP_FirstPersonCharacter.KeycardColor` _asbp_first_person_character) _doorcolor)
      _
      (else
        (return false))))
  (return true))

(fn `UserConstructionScript`
  (bind _box (`self.Box`))
  (if (`self.ClosingTriggerBox`)
    (`BoxComponent.SetBoxExtent` _box (70.0 70.0 70.0) true)
    (else
      (`BoxComponent.SetBoxExtent` _box (0.0 0.0 0.0) true))))