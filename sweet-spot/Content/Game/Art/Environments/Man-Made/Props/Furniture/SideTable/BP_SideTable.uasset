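; Side table prop with a drawer that the first-person character can open and close by interacting.
; Each successful interaction plays a 2D switch sound and flip-flops a timeline forward or in reverse, sliding the drawer mesh along its local Y axis.
; The drawer mesh's collision is disabled at BeginPlay.
; The construction script applies an optional Symbol material to a decal.
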(event `self.ReceiveBeginPlay`
  (`PrimitiveComponent.SetCollisionEnabled` (`self.StaticMesh2`) "NoCollision"))

(event `/Game/Jason/Interface/BPI_InteractInterface.InteractSuccess`
  (params (InteractingCaller :type "Actor Object Reference"))
  (`FMODBlueprintStatics.PlayEvent2D` "/Game/FMOD/Events/SFX/Switches.Switches")
  (`/Engine/EditorBlueprintResources/StandardMacros.FlipFlop`
    (:`A`
      (bind (_direction _openamount) (`Timeline|OpenDrawer` :!label _label)
        (:`Update`
          (`SceneComponent.K2_SetRelativeLocation` (`self.StaticMesh2`) (`KismetMathLibrary.MakeVector` 0.0 (* _openamount 25.0)) false false))))
    (:`B`
      (goto _label :!via `Reverse`))))

(fn `CanInteract`
  (params (InteractingActor :type "Actor Object Reference"))
  (returns (CanInteract :type Boolean))
  (cast `/Game/FirstPerson/Blueprints/BP_FirstPersonCharacter` InteractingActor)
  (return true))

(fn `UserConstructionScript`
  (bind _symbol (`self.Symbol`))
  (`/Engine/EditorBlueprintResources/StandardMacros.IsValid` _symbol
    (:`Is Valid`
      (`DecalComponent.SetDecalMaterial` (`self.e`) _symbol))))