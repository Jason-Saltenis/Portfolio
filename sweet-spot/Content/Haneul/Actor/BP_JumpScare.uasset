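; One-shot jump scare trigger actor that fires when the first-person player walks into its collision component.
; An overlap from the character's capsule plays the PopupKey FMOD event at the actor's location and adds the WBP_JumpScare widget to the viewport.
; After a delay set by the Time variable, it removes the widget and destroys itself.
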(event `self.CollisionComponent.OnComponentBeginOverlap`
  (params (OverlappedComponent :type "PrimitiveComponent Object Reference") (OtherActor :type "Actor Object Reference") (OtherComp :type "PrimitiveComponent Object Reference") (OtherBodyIndex :type Integer) (bFromSweep :type Boolean) (SweepResult :type "HitResult Structure (by ref)"))
  (cast `CapsuleComponent` OtherComp)
  (cast `/Game/FirstPerson/Blueprints/BP_FirstPersonCharacter` OtherActor)
  (`FMODBlueprintStatics.PlayEventAtLocation` "/Game/FMOD/Events/SFX/PopupKey.PopupKey" (`KismetMathLibrary.Conv_VectorToTransform` (`self.K2_GetActorLocation` self)))
  (bind _returnvalue (`|CreateWidget` "/Game/Haneul/Widget/WBP_JumpScare.WBP_JumpScare_C"))
  (`UserWidget.AddToViewport` _returnvalue 0)
  (`KismetSystemLibrary.Delay` (`self.time`))
  (`Widget.RemoveFromParent` _returnvalue)
  (`self.K2_DestroyActor`))

(fn `UserConstructionScript`)