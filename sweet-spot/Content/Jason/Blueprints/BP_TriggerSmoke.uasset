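; Box trigger actor that holds logic for toggling a BP_Smoke actor attached to the first-person character.
; Begin overlap casts to the character and, if the madness meter is exactly full, detaches and destroys the trigger itself.
; End overlap feeds only a DoOnce's Reset input; that node's Completed branch removes existing smoke or spawns and snaps new smoke onto the cast character.
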(event `self.Box.OnComponentBeginOverlap`
  (params (OverlappedComponent :type "PrimitiveComponent Object Reference") (OtherActor :type "Actor Object Reference") (OtherComp :type "PrimitiveComponent Object Reference") (OtherBodyIndex :type Integer) (bFromSweep :type Boolean) (SweepResult :type "HitResult Structure (by ref)"))
  (bind _asbp_first_person_character (cast `/Game/FirstPerson/Blueprints/BP_FirstPersonCharacter` OtherActor))
  (if (== (`MyUserWidget.currentMadnessBarValue` (`self.MadnessMeter`)) 1.0)
    (`self.K2_DetachFromActor` "KeepRelative")
    (`self.K2_DestroyActor`)))

(event `self.Box.OnComponentEndOverlap`
  (params (OverlappedComponent :type "PrimitiveComponent Object Reference") (OtherActor :type "Actor Object Reference") (OtherComp :type "PrimitiveComponent Object Reference") (OtherBodyIndex :type Integer))
  (bind _var_bp_smoke (`self.var_bp_smoke`))
  (`/Engine/EditorBlueprintResources/StandardMacros.DoOnce` false :!via `Reset`
    (:`Completed`
      (if (`KismetSystemLibrary.IsValid` _var_bp_smoke)
        (`self.K2_DetachFromActor` _var_bp_smoke "KeepRelative" "KeepRelative" "KeepRelative")
        (`self.K2_DestroyActor` _var_bp_smoke)
        (else
          (bind _returnvalue (`|SpawnActorFromClass` "/Game/Jason/Blueprints/BP_Smoke.BP_Smoke_C" (`self.GetTransform` (stale `self.Box.OnComponentBeginOverlap` _asbp_first_person_character)) "AlwaysSpawn" "MultiplyWithRoot" null (0.0 0.0 0.0) 0.2 0.8 null))
          (bind _output_get (set `self.var_bp_smoke` _returnvalue))
          (`self.K2_AttachToActor` _output_get (stale `self.Box.OnComponentBeginOverlap` _asbp_first_person_character) "None" "SnapToTarget" "KeepRelative" "KeepRelative" true))))))

(fn `UserConstructionScript`)