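; Tentacle Blueprint that procedurally animates a skeletal mesh through a Control Rig component.
; On rig pre-initialize it maps the mesh as output, caches control positions and seeds random noise offsets per control.
; A looping timer of about 60 Hz moves each control by time-based Perlin noise plus a Y-Z coil offset.
; Curves sampled along the control chain shape noise amount and coil radius; a socket attach node is left unconnected.
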(event `self.ControlRig.OnPreInitializeDelegate`
  (params (Component :type "ControlRigComponent Object Reference"))
  (bind _offsets (`self.Offsets`))
  (`ControlRigComponent.AddMappedCompleteSkeletalMesh` Component (`self.SkeletalMesh`) "Output")
  (for (_ _array_index) _offsets
    (`KismetArrayLibrary.Array_Set` _offsets _array_index (* (`KismetMathLibrary.RandomUnitVector`) (10.0 10.0 10.0)))
    (`KismetArrayLibrary.Array_Set` (`self.InitialPositions`) _array_index (`ControlRigComponent.GetControlPosition` (`self.ControlRig`) (`|GetArrayItem` (`self.ControlNames`) _array_index) "LocalSpace") true)))

(event `self.ReceiveBeginPlay`
  (`KismetSystemLibrary.K2_SetTimerDelegate` (delegate `TentacleMoving`) 0.016 true))

(event `TentacleMoving`
  (bind _controlnames (`self.ControlNames`))
  (bind _returnvalue (* (`KismetSystemLibrary.GetGameTimeInSeconds`) 1.0))
  (bind _returnvalue_2 (- (`KismetArrayLibrary.Array_Length` _controlnames) 1))
  (for _index (range (+ _returnvalue_2 1))
    (bind _output_x (`KismetMathLibrary.BreakVector` (`|GetArrayItem` (`self.Offsets`) _index)))
    (bind (_output_x_2 _output_y) (`KismetMathLibrary.BreakVector` (`|GetArrayItem` (`self.Offsets`) _index)))
    (bind (_output_x_3 _output_y_2 _output_z) (`KismetMathLibrary.BreakVector` (`|GetArrayItem` (`self.Offsets`) _index)))
    (bind _returnvalue_3 (/ (`KismetMathLibrary.Conv_IntToDouble` _index) (`KismetMathLibrary.Conv_IntToDouble` _returnvalue_2)))
    (bind _returnvalue_4 (* _returnvalue_3 (`self.CoilAngle`)))
    (`ControlRigComponent.SetControlPosition` (`self.ControlRig`) (`|GetArrayItem` _controlnames _index) (+ (* (* (`KismetMathLibrary.MakeVector` (`KismetMathLibrary.PerlinNoise1D` (+ _returnvalue _output_x)) (`KismetMathLibrary.PerlinNoise1D` (+ _returnvalue _output_y)) (`KismetMathLibrary.PerlinNoise1D` (+ _returnvalue _output_z))) (`CurveFloat.GetFloatValue` (`self.NoiseCurve`) _returnvalue_3)) (`self.NoiseStrength`)) (+ (`|GetArrayItem` (`self.InitialPositions`) _index) (* (`KismetMathLibrary.MakeVector` 0.0 (`KismetMathLibrary.DegCos` _returnvalue_4) (`KismetMathLibrary.DegSin` _returnvalue_4)) (* (`self.Radius`) (`CurveFloat.GetFloatValue` (`self.RadiusCurve`) _returnvalue_3))))) "LocalSpace")))

(fn `UserConstructionScript`)