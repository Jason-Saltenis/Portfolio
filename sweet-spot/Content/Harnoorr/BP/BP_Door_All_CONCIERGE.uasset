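; Concierge door Blueprint that allows interaction only when the player's keycard color matches the door's color.
; CanInteract casts the interacting actor to BP_FirstPersonCharacter and compares its KeycardColor with DoorColor.
; KeycardCheck is an empty function with disconnected leftover nodes for granting a keycard and printing its color gameplay tag.
; The file contains no logic for opening the door.
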(fn `CanInteract`
  (params (InteractingActor :type "Actor Object Reference"))
  (returns (CanInteract :type Boolean))
  (bind _asbp_first_person_character (cast `/Game/FirstPerson/Blueprints/BP_FirstPersonCharacter` InteractingActor))
  (return (== (`/Game/FirstPerson/Blueprints/BP_FirstPersonCharacter.KeycardColor` _asbp_first_person_character) (`self.DoorColor`))))

(fn `Keycard_Check`)

(fn `UserConstructionScript`)