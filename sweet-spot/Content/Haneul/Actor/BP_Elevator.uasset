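; Interactable elevator that drives the crash cutscene, the repair objective and the final cutscene.
; While a BP_CutSceneEnd exists, it locks doors; interacting plays the Crash sequence and teleports the player there, then restores doors and hides the crank, switch and button.
; Otherwise interaction calls FixElevator, sparking until all three parts show, and fires BP_TriggerCutscene's final cutscene if present.
; An optional one-shot trigger box lights the hall lights.
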(event `SetUpElevator`
  (bind _elevator_plate (`self.Elevator_Plate`))
  (bind _niagara (`self.Niagara`))
  (bind _elevator_plate_2 (`self.Elevator_Plate`))
  (`self.ShowParts`)
  (if (`self.SparksOn`)
    (`ActorComponent.Activate` _niagara false)
    (else
      (`ActorComponent.Deactivate` _niagara)))
  (bind _returnvalue (`GameplayStatics.GetActorOfClass` "/Game/Haneul/Actor/BP_CutSceneEnd.BP_CutSceneEnd_C"))
  (bind _output_get (set `self.TeleportActor` _returnvalue))
  (`/Engine/EditorBlueprintResources/StandardMacros.IsValid` _output_get
    (:`Is Valid`
      (`PrimitiveComponent.SetCollisionEnabled` _elevator_plate "QueryAndPhysics")
      (`PrimitiveComponent.SetCollisionEnabled` (`self.Cube`) "QueryAndPhysics")
      (`self.CloseAllDoors`))
    (:`Is Not Valid`
      (`PrimitiveComponent.SetCollisionEnabled` _elevator_plate "NoCollision")
      (`PrimitiveComponent.SetCollisionEnabled` (`self.Cube`) "NoCollision")
      (bind _returnvalue_2 (`GameplayStatics.GetActorOfClass` "/Game/Blueprints/BP_TriggerCutscene.BP_TriggerCutscene_C"))
      (bind _output_get_2 (set `self.FinalCutScene` _returnvalue_2))
      (`/Engine/EditorBlueprintResources/StandardMacros.IsValid` _output_get_2
        (:`Is Valid`
          (`PrimitiveComponent.SetCollisionEnabled` _elevator_plate_2 "QueryAndPhysics")
          (`PrimitiveComponent.SetCollisionEnabled` (`self.Cube`) "QueryAndPhysics"))
        (:`Is Not Valid`
          (`PrimitiveComponent.SetCollisionEnabled` _elevator_plate_2 "NoCollision")
          (`PrimitiveComponent.SetCollisionEnabled` (`self.Cube`) "NoCollision"))))))

(event `self.Exit`
  (bind _exitref (`self.ExitRef`))
  (`/Engine/EditorBlueprintResources/StandardMacros.IsValid` _exitref
    (:`Is Valid`
      (`/Game/Harnoorr/BP/BP_EXIT.TurnLightOn` _exitref))))

(event `/Game/Jason/Interface/BPI_InteractInterface.InteractSuccess`
  (params (InteractingCaller :type "Actor Object Reference"))
  (bind _finalcutscene (`self.FinalCutScene`))
  (`/Engine/EditorBlueprintResources/StandardMacros.IsValid` _finalcutscene
    (:`Is Valid`
      (`/Game/Blueprints/BP_TriggerCutscene.FinalCutScene` _finalcutscene)
      (`self.K2_DestroyActor` (`self.ExitRef`)))
    (:`Is Not Valid`
      _))
  (`PrimitiveComponent.SetCollisionEnabled` (`self.Elevator_Plate`) "NoCollision")
  (`PrimitiveComponent.SetCollisionEnabled` (`self.Cube`) "NoCollision")
  (`PrimitiveComponent.SetCustomDepthStencilValue` (`self.Elevator_Plate`) 0)
  (`/Engine/EditorBlueprintResources/StandardMacros.IsValid` (`self.TeleportActor`)
    (:`Is Valid`
      ; Cut Scene
      (bind _asbp_first_person_character (cast `/Game/FirstPerson/Blueprints/BP_FirstPersonCharacter` (`GameplayStatics.GetPlayerCharacter` 0)))
      (`SceneComponent.SetVisibility` (`/Game/FirstPerson/Blueprints/BP_FirstPersonCharacter.Arm` _asbp_first_person_character) false false)
      (`self.DisableInput` (`GameplayStatics.GetPlayerCharacter` 0) (`GameplayStatics.GetPlayerController` 0))
      (bind _outactor (`LevelSequencePlayer.CreateLevelSequencePlayer` (`self.Crash`)))
      (bind _sequenceplayer (`LevelSequenceActor.SequencePlayer` _outactor))
      (`MovieSceneSequencePlayer.Play` _sequenceplayer)
      (`FMODBlueprintStatics.PlayEventAtLocation` "/Game/FMOD/Events/SFX/ElevatorFailure.ElevatorFailure" (`self.GetTransform` (`GameplayStatics.GetPlayerPawn` 0)))
      (add `MovieSceneSequencePlayer.OnFinished` _sequenceplayer (delegate `OnSequenceFinished`))
      (`self.TeleportPlayerToArrow`)
      (bind _asbp_first_person_character_2 (cast `/Game/FirstPerson/Blueprints/BP_FirstPersonCharacter` (`GameplayStatics.GetPlayerPawn` 0)))
      (`Widget.SetVisibility` (`/Game/FirstPerson/Blueprints/BP_FirstPersonCharacter.AimRef` _asbp_first_person_character_2) "Collapsed"))
    (:`Is Not Valid`
      (`self.FixElevator`)
      (bind _asplayer_hud (cast `PlayerHud` (`PlayerController.GetHUD` (`GameplayStatics.GetPlayerController` 0))))
      (bind _aswbp_pop_up (cast `/Game/Haneul/Widget/WBP_PopUp` (`PlayerHud.PopUpWidget` _asplayer_hud)))
      (`/Game/Haneul/Widget/WBP_PopUp.ElevatorPeice` _aswbp_pop_up null)
      (`self.Sparks`))))

(event `OnSequenceFinished`
  ; Cut Scene
  (`self.End CutScene`)
  (`self.ResetAllDoors`)
  (`PrimitiveComponent.SetCollisionEnabled` (`self.TurnLightsOn`) "QueryAndPhysics")
  (`self.SetUpElevator`)
  (`self.Sparks`))

(event `self.TurnLightsOn.OnComponentBeginOverlap`
  (params (OverlappedComponent :type "PrimitiveComponent Object Reference") (OtherActor :type "Actor Object Reference") (OtherComp :type "PrimitiveComponent Object Reference") (OtherBodyIndex :type Integer) (bFromSweep :type Boolean) (SweepResult :type "HitResult Structure (by ref)"))
  (cast `/Game/FirstPerson/Blueprints/BP_FirstPersonCharacter` OtherActor)
  (bind _outactors (`GameplayStatics.GetAllActorsOfClass` "/Game/Harnoorr/BP/BP_NEW/BP_HallLight.BP_HallLight_C"))
  (for _array_element _outactors
    (`PrimitiveComponent.SetMaterial` (`/Game/Harnoorr/BP/BP_NEW/BP_HallLight.Light` _array_element) 1 "/Game/Jason/MATs/MAT_Cores/M_emissive_Base.M_emissive_Base")
    (`LightComponent.SetIntensity` (`/Game/Harnoorr/BP/BP_NEW/BP_HallLight.SpotLight` _array_element) 30.0)
    (`LightComponent.SetIntensity` (`/Game/Harnoorr/BP/BP_NEW/BP_HallLight.SpotLight1` _array_element) 30.0))
  (`ActorComponent.K2_DestroyComponent` (`self.TurnLightsOn`)))

(fn `CanInteract`
  (params (InteractingActor :type "Actor Object Reference"))
  (returns (CanInteract :type Boolean))
  (cast `/Game/FirstPerson/Blueprints/BP_FirstPersonCharacter` InteractingActor)
  (return true))

(fn `CloseAllDoors`
  (bind _outactors (`GameplayStatics.GetAllActorsOfClass` "/Game/Harnoorr/BP/BP_NEW/BP_NEW_DOOR_COPY.BP_NEW_DOOR_COPY_C"))
  (bind _output_get (set `self.Door` _outactors))
  (for _array_element _output_get
    (`KismetArrayLibrary.Array_Add` (`self.originalDoorColor`) (`/Game/Harnoorr/BP/BP_NEW/BP_NEW_DOOR_COPY.DoorColor` _array_element))
    (set `/Game/Harnoorr/BP/BP_NEW/BP_NEW_DOOR_COPY.DoorColor` (struct :`TagName` "SweetSpot.KeyCard.Color.Lock") _array_element))
  (bind _returnvalue (`GameplayStatics.GetActorOfClass` "/Game/Harnoorr/BP/BP_NEW/BP_TEST_DOOR.BP_TEST_DOOR_C"))
  (`PrimitiveComponent.SetCollisionEnabled` (`/Game/Harnoorr/BP/BP_NEW/BP_TEST_DOOR.OpenDoorTriggerbox` _returnvalue) "NoCollision"))

(fn `End CutScene`
  (bind _returnvalue (`GameplayStatics.GetPlayerCharacter` 0))
  (bind _returnvalue_2 (`GameplayStatics.GetPlayerController` 0))
  (`self.EnableInput` _returnvalue _returnvalue_2)
  (`PlayerController.SetViewTargetWithBlend` _returnvalue_2 _returnvalue 1.0 "VTBlend_Linear" 0.0 false)
  (`SceneComponent.SetVisibility` (`self.Switch`) false false)
  (`SceneComponent.SetVisibility` (`self.Button`) false false)
  (`SceneComponent.SetVisibility` (`self.Cranck`) false false)
  (`self.Sparks`)
  (`self.K2_DestroyActor` (`self.TeleportActor`))
  (bind _asbp_first_person_character (cast `/Game/FirstPerson/Blueprints/BP_FirstPersonCharacter` (`GameplayStatics.GetPlayerCharacter` 0)))
  (`SceneComponent.SetVisibility` (`/Game/FirstPerson/Blueprints/BP_FirstPersonCharacter.Arm` _asbp_first_person_character) true false)
  (bind _asbp_first_person_character_2 (cast `/Game/FirstPerson/Blueprints/BP_FirstPersonCharacter` (`GameplayStatics.GetPlayerPawn` 0)))
  (`Widget.SetVisibility` (`/Game/FirstPerson/Blueprints/BP_FirstPersonCharacter.AimRef` _asbp_first_person_character_2) "Visible"))

(fn `ResetAllDoors`
  (for (_array_element _array_index) (`self.Door`)
    (set `/Game/Harnoorr/BP/BP_NEW/BP_NEW_DOOR_COPY.DoorColor` (`|GetArrayItem` (`self.originalDoorColor`) _array_index) _array_element))
  (bind _returnvalue (`GameplayStatics.GetActorOfClass` "/Game/Harnoorr/BP/BP_NEW/BP_TEST_DOOR.BP_TEST_DOOR_C"))
  (`PrimitiveComponent.SetCollisionEnabled` (`/Game/Harnoorr/BP/BP_NEW/BP_TEST_DOOR.OpenDoorTriggerbox` _returnvalue) "QueryAndPhysics"))

(fn `ShowParts`
  (bind _switch (`self.Switch`))
  (bind _cranck (`self.Cranck`))
  (bind _button (`self.Button`))
  (`self.SetChildPart` _cranck "Cranck")
  (bind _asbp_elevator_part (cast `/Game/Haneul/Actor/BP_ElevatorPart` (`ChildActorComponent.ChildActor` _cranck)))
  (`/Game/Haneul/Actor/BP_ElevatorPart.SetMesh` _asbp_elevator_part)
  (`self.SetChildPart` _switch "Switch")
  (bind _asbp_elevator_part_2 (cast `/Game/Haneul/Actor/BP_ElevatorPart` (`ChildActorComponent.ChildActor` _switch)))
  (`/Game/Haneul/Actor/BP_ElevatorPart.SetMesh` _asbp_elevator_part_2)
  (`self.SetChildPart` _button "Button")
  (bind _asbp_elevator_part_3 (cast `/Game/Haneul/Actor/BP_ElevatorPart` (`ChildActorComponent.ChildActor` _button)))
  (`/Game/Haneul/Actor/BP_ElevatorPart.SetMesh` _asbp_elevator_part_3))

(fn `Sparks`
  (bind _niagara (`self.Niagara`))
  (if (and (and (`SceneComponent.IsVisible` (`self.Switch`)) (`SceneComponent.IsVisible` (`self.Button`))) (`SceneComponent.IsVisible` (`self.Cranck`)))
    (`ActorComponent.Deactivate` _niagara)
    (else
      (`ActorComponent.Activate` _niagara false))))

(fn `TeleportPlayerToArrow`
  (`self.K2_SetActorLocation` (`GameplayStatics.GetPlayerCharacter` 0) (`self.K2_GetActorLocation` (`self.TeleportActor`)) false true)
  (`Controller.SetControlRotation` (`GameplayStatics.GetPlayerController` 0) (`SceneComponent.K2_GetComponentRotation` (`/Game/Haneul/Actor/BP_CutSceneEnd.Arrow` (`self.TeleportActor`)))))

(fn `UserConstructionScript`
  (bind _turnlightson (`self.TurnLightsOn`))
  (`self.ShowParts`)
  (`PrimitiveComponent.SetCollisionEnabled` (`self.Elevator_Plate`) "NoCollision")
  (`PrimitiveComponent.SetCollisionEnabled` (`self.TurnLightsOn`) "NoCollision")
  (`PrimitiveComponent.SetCollisionEnabled` (`self.Cube`) "NoCollision")
  (if (`self.TurnOnLightTriggerbox`)
    (`BoxComponent.SetBoxExtent` _turnlightson (100.0 100.0 100.0) true)
    (else
      (`BoxComponent.SetBoxExtent` _turnlightson (0.0 0.0 0.0) true))))