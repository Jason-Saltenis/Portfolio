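; BP_ElevatorPart is an elevator component actor that displays as a switch, button or crank.
; The ElevatorPart enum picks the Cube mesh, with None falling back to the switch; the construction script and SetMesh, called on BeginPlay, duplicate this logic.
; CanInteract casts the interacting actor to BP_FirstPersonCharacter but returns false even when the cast succeeds.
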(event `self.ReceiveBeginPlay`
  (`self.SetMesh`))

(fn `CanInteract`
  (params (InteractingActor :type "Actor Object Reference"))
  (returns (CanInteract :type Boolean))
  (cast `/Game/FirstPerson/Blueprints/BP_FirstPersonCharacter` InteractingActor)
  (return false))

(fn `SetMesh`
  (switch `EElevatorPart` (`self.ElevatorPart`)
    (:`None`
      (`StaticMeshComponent.SetStaticMesh` (`self.Cube`) "/Game/Game/Art/Environments/Man-Made/Props/Elevator/Switch.Switch" :!label _label))
    (:`Switch`
      (goto _label))
    (:`Button`
      (`StaticMeshComponent.SetStaticMesh` (`self.Cube`) "/Game/Game/Art/Environments/Man-Made/Props/Elevator/Button.Button"))
    (:`Cranck`
      (`StaticMeshComponent.SetStaticMesh` (`self.Cube`) "/Game/Game/Art/Environments/Man-Made/Props/Elevator/Crank.Crank"))))

(fn `UserConstructionScript`
  (switch `EElevatorPart` (`self.ElevatorPart`)
    (:`None`
      (`StaticMeshComponent.SetStaticMesh` (`self.Cube`) "/Game/Game/Art/Environments/Man-Made/Props/Elevator/Switch.Switch" :!label _label))
    (:`Switch`
      (goto _label))
    (:`Button`
      (`StaticMeshComponent.SetStaticMesh` (`self.Cube`) "/Game/Game/Art/Environments/Man-Made/Props/Elevator/Button.Button"))
    (:`Cranck`
      (`StaticMeshComponent.SetStaticMesh` (`self.Cube`) "/Game/Game/Art/Environments/Man-Made/Props/Elevator/Crank.Crank"))))