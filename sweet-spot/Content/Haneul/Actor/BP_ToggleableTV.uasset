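; BP_ToggleableTV is an interactable television that the first-person character can switch on and off.
; A successful interaction flips IsOn through TurnTVOn or TurnTVOff, and initialize applies the starting state.
; These functions toggle the spotlight, TV sound, screen material and TriggerBox collision, and play a 2D button sound event.
; CanInteract accepts only BP_FirstPersonCharacter and returns IsInteractable.
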(event `initialize`
  (if (`self.isOn`)
    (`self.TurnTVOn`)
    (else
      (`self.TurnTVOff`))))

(event `self.ReceiveBeginPlay`)

(event `/Game/Jason/Interface/BPI_InteractInterface.InteractSuccess`
  (params (InteractingCaller :type "Actor Object Reference"))
  (if (`self.isOn`)
    (`self.TurnTVOff`)
    (else
      (`self.TurnTVOn`))))

(fn `CanInteract`
  (params (InteractingActor :type "Actor Object Reference"))
  (returns (CanInteract :type Boolean))
  (cast `/Game/FirstPerson/Blueprints/BP_FirstPersonCharacter` InteractingActor)
  (return (`self.isInteractable`)))

(fn `TurnTVOff`
  (set `self.isOn` false)
  (`PrimitiveComponent.SetCollisionEnabled` (`self.triggerBox`) "NoCollision")
  (`SceneComponent.SetVisibility` (`self.SpotLight`) false false)
  (`FMODAudioComponent.Stop` (`self.SFX_TV`))
  (`PrimitiveComponent.SetMaterial` (`self.TV`) 2 (`self.ScreenMaterialOff`))
  (`FMODBlueprintStatics.PlayEvent2D` "/Game/FMOD/Events/SFX/Buttons.Buttons"))

(fn `TurnTVOn`
  (set `self.isOn` true)
  (`PrimitiveComponent.SetCollisionEnabled` (`self.triggerBox`) "QueryAndPhysics")
  (`SceneComponent.SetVisibility` (`self.SpotLight`) true false)
  (`SceneComponent.SetVisibility` (`self.SFX_TV`) true false)
  (`FMODAudioComponent.Play` (`self.SFX_TV`))
  (`PrimitiveComponent.SetMaterial` (`self.TV`) 2 (`self.ScreenMaterialOn`))
  (`FMODBlueprintStatics.PlayEvent2D` "/Game/FMOD/Events/SFX/Buttons.Buttons"))

(fn `UserConstructionScript`)