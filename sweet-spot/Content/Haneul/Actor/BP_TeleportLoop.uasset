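; BP_TeleportLoop is an actor that moves the player on to the next loop level.
; When LoadSubLevel fires and the loop is completed, it stream-loads the soft-referenced NextLoopLevel with a blocking load, then teleports the player's pawn using NextArrow.
; It then passes ThisLoopLevel to SweetSpotGameMode's CheckForSubLevel.
; If no valid next level is set, it opens the MM_Credits level instead.
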(event `self.ReceiveBeginPlay`)

(event `self.ReceiveActorBeginOverlap`
  (params (OtherActor :type "Actor Object Reference")))

(event `self.LoadSubLevel`
  (if (`self.isCompleted`)
    (if (`KismetSystemLibrary.IsValidSoftObjectReference` (`self.NextLoopLevel`))
      (`GameplayStatics.LoadStreamLevelBySoftObjectPtr` (`self.NextLoopLevel`) true true)
      (`self.Teleport` (`Controller.K2_GetPawn` (`GameplayStatics.GetPlayerController` 0)) (`self.nextArrow`))
      (bind _assweet_spot_game_mode (cast `SweetSpotGameMode` (`GameplayStatics.GetGameMode`)))
      (`SweetSpotGameMode.CheckForSubLevel` _assweet_spot_game_mode (`self.thisLoopLevel`))
      (else
        (`GameplayStatics.OpenLevelBySoftObjectPtr` "/Game/Game/Levels/UI/MM_Credits.MM_Credits")))))

(fn `UserConstructionScript`)