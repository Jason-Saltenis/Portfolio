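; BP_BigEye is an eye actor that can turn to face the player's first-person camera and close or reopen its eyelids.
; LookatPlayer rotates the root toward the camera, while FadeAway calls CloseEye when Count is 1 and ResetPosition calls OpenEye.
; CloseEye plays eye and eyelid animations, then after a short delay pins them at a fixed position and pauses them.
; OpenEye simply unpauses those same animations.
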(event `self.LookAtPlayer`
  (bind _defaultsceneroot (`self.DefaultSceneRoot`))
  (bind _asbp_first_person_character (cast `/Game/FirstPerson/Blueprints/BP_FirstPersonCharacter` (`Controller.K2_GetPawn` (`GameplayStatics.GetPlayerController` 0))))
  (`SceneComponent.K2_SetWorldRotation` _defaultsceneroot (`KismetMathLibrary.FindLookAtRotation` (`SceneComponent.K2_GetComponentLocation` _defaultsceneroot) (`SceneComponent.K2_GetComponentLocation` (`/Game/FirstPerson/Blueprints/BP_FirstPersonCharacter.FirstPersonCamera` _asbp_first_person_character))) false false))

(event `CustomEvent`
  (bind _eye (`self.Eye`))
  (`KismetSystemLibrary.Delay` 0.2)
  (`SkeletalMeshComponent.SetPosition` _eye 0.2 true)
  (`SkeletalMeshComponent.SetPosition` (`self.EyelidLower_low`) 0.2 true)
  (`SkeletalMeshComponent.SetPosition` (`self.EyelidHigher_low`) 0.2 true)
  (set `SkeletalMeshComponent.bPauseAnims` true _eye)
  (set `SkeletalMeshComponent.bPauseAnims` true (`self.EyelidHigher_low`))
  (set `SkeletalMeshComponent.bPauseAnims` true (`self.EyelidLower_low`)))

(event `self.FadeAway`
  (if (== (`self.count`) 1)
    (`self.CloseEye`)))

(event `self.ResetPosition`
  (`self.OpenEye`))

(fn `CloseEye`
  (`SkeletalMeshComponent.PlayAnimation` (`self.Eye`) "/Game/Game/Art/Characters/Model/Eyeball/Eyeshells/Eyeshell01/Eyeshell01_low_Anim.Eyeshell01_low_Anim" false)
  (`SkeletalMeshComponent.PlayAnimation` (`self.EyelidLower_low`) "/Game/Game/Art/Characters/Model/Eyeball/Eyelids/EyelidLower/EyelidLower_low_Anim.EyelidLower_low_Anim" false)
  (`SkeletalMeshComponent.PlayAnimation` (`self.EyelidHigher_low`) "/Game/Game/Art/Characters/Model/Eyeball/Eyelids/EyelidHigher/EyelidHigher_low_Anim.EyelidHigher_low_Anim" false)
  (`self.CustomEvent`))

(fn `OpenEye`
  (set `SkeletalMeshComponent.bPauseAnims` false (`self.Eye`))
  (set `SkeletalMeshComponent.bPauseAnims` false (`self.EyelidHigher_low`))
  (set `SkeletalMeshComponent.bPauseAnims` false (`self.EyelidLower_low`)))

(fn `UserConstructionScript`)