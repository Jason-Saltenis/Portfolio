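; Interactable elevator part pickup (switch, button or crank) that only the first-person character can collect.
; The construction script sets mesh, offset and popup image from the ElevatorPart enum.
; On interaction it adds the part to the player's inventory, plays a sound event, enables query collision and custom-depth stencil on the elevator's plate, and shows the HUD popup.
; It then unhides linked Door actors, pausing their portal SFX, and destroys itself.
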(event `/Game/Jason/Interface/BPI_InteractInterface.InteractSuccess`
  (params (InteractingCaller :type "Actor Object Reference"))
  (bind _asbp_first_person_character (cast `/Game/FirstPerson/Blueprints/BP_FirstPersonCharacter` InteractingCaller))
  (`PlayerInventory.GetElevatorPart` (`/Game/FirstPerson/Blueprints/BP_FirstPersonCharacter.PlayerInventory` _asbp_first_person_character) (`self.ElevatorPart`))
  (`FMODBlueprintStatics.PlayEventAtLocation` "/Game/FMOD/Events/UI/ButtonPress.ButtonPress" (`KismetMathLibrary.Conv_VectorToTransform` (`self.K2_GetActorLocation` self)))
  (`self.UpdateElevatorPlate`)
  (bind _asplayer_hud (cast `PlayerHud` (`PlayerController.GetHUD` (`GameplayStatics.GetPlayerController` 0))))
  (bind _aswbp_pop_up (cast `/Game/Haneul/Widget/WBP_PopUp` (`PlayerHud.PopUpWidget` _asplayer_hud)))
  (`/Game/Haneul/Widget/WBP_PopUp.ElevatorPeice` _aswbp_pop_up (`self.Img`))
  (`self.ShowDoor`)
  (`self.K2_DestroyActor`))

(fn `CanInteract`
  (params (InteractingActor :type "Actor Object Reference"))
  (returns (CanInteract :type Boolean))
  (cast `/Game/FirstPerson/Blueprints/BP_FirstPersonCharacter` InteractingActor)
  (return true))

(fn `HideDoor`
  (for _array_element (`self.Door`)
    (`/Engine/EditorBlueprintResources/StandardMacros.IsValid` _array_element
      (:`Is Valid`
        (`self.SetActorHiddenInGame` _array_element true)
        (`FMODAudioComponent.SetPaused` (`/Game/Haneul/Actor/BP_TeleportDoor.SFX_Portal` _array_element) false)))))

(fn `SetUpPart`
  (bind _staticmesh (`self.StaticMesh`))
  (switch `EElevatorPart` (`self.ElevatorPart`)
    (:`None`
      (`StaticMeshComponent.SetStaticMesh` _staticmesh "/Game/Game/Art/Environments/Man-Made/Props/Elevator/Switch.Switch" :!label _label)
      (`SceneComponent.K2_SetRelativeLocation` (`self.StaticMesh`) (-15.0 0.0 -15.0) false false)
      (set `self.Img` "/Game/Haneul/FinalSwitch_IMG.FinalSwitch_IMG"))
    (:`Switch`
      (goto _label))
    (:`Button`
      (`StaticMeshComponent.SetStaticMesh` _staticmesh "/Game/Game/Art/Environments/Man-Made/Props/Elevator/Button.Button")
      (`SceneComponent.K2_SetRelativeLocation` (`self.StaticMesh`) (15.0 0.0 -15.0) false false)
      (set `self.Img` "/Game/Haneul/FinalButton_IMG.FinalButton_IMG"))
    (:`Cranck`
      (`StaticMeshComponent.SetStaticMesh` _staticmesh "/Game/Game/Art/Environments/Man-Made/Props/Elevator/Crank.Crank")
      (`SceneComponent.K2_SetRelativeLocation` (`self.StaticMesh`) (0.0 0.0 -30.0) false false)
      (set `self.Img` "/Game/Haneul/FinalCrank_IMG.FinalCrank_IMG"))))

(fn `ShowDoor`
  (for _array_element (`self.Door`)
    (`/Engine/EditorBlueprintResources/StandardMacros.IsValid` _array_element
      (:`Is Valid`
        (`self.SetActorHiddenInGame` _array_element false)
        (`FMODAudioComponent.SetPaused` (`/Game/Haneul/Actor/BP_TeleportDoor.SFX_Portal` _array_element) true)))))

(fn `UpdateElevatorPlate`
  (bind _outactors (`GameplayStatics.GetAllActorsOfClass` "/Game/Haneul/Actor/BP_Elevator.BP_Elevator_C"))
  (bind _elevator_plate (`/Game/Haneul/Actor/BP_Elevator.Elevator_Plate` (`|GetArrayItem` _outactors)))
  (`PrimitiveComponent.SetCustomDepthStencilValue` _elevator_plate 1)
  (`PrimitiveComponent.SetCollisionEnabled` _elevator_plate "QueryOnly"))

(fn `UserConstructionScript`
  (`self.SetUpPart`))