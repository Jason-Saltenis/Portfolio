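; BP_PlayerLook picks the interactable actor the player is looking at from those inside a supplied collision sphere.
; LookForActor gathers the sphere's overlapping actors that implement BPI_InteractInterface and passes them to LookAtActor, whose body is not shown.
; It then clears the candidate array and returns the chosen actor, with BeginPlay and Tick left unused.
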(fn `LookForActor`
  (params (`Sphere Collision` :type "SphereComponent Object Reference"))
  (returns (isInteractable :type "Actor Object Reference"))
  (for _array_element (`PrimitiveComponent.GetOverlappingActors` `Sphere Collision` "/Script/Engine.Actor")
    (if (`KismetSystemLibrary.DoesImplementInterface` _array_element "/Game/Jason/Interface/BPI_InteractInterface.BPI_InteractInterface_C")
      (`KismetArrayLibrary.Array_Add` (`self.InteractableActor`) _array_element)))
  (bind _returnvalue (`self.LookAtActor` (`self.InteractableActor`)))
  (`KismetArrayLibrary.Array_Clear` (`self.InteractableActor`))
  (return _returnvalue))