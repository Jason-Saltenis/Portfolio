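; Interactable hinged door with a room nameplate chosen by number in the construction script and an optional keycard color lock.
; CanInteract checks the first-person character's keycard against DoorColor; failure plays a knob rattle at the door.
; Success or OpenDoor/CloseDoor calls run LockDoor, which toggles state, plays a creak or close sound, and drives a Timeline forward or backward to rotate door and handle.
; Door collision is disabled during the swing and restored when the Timeline finishes.
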(event `LockDoor`
  (`PrimitiveComponent.SetCollisionEnabled` (`self.DOOR`) "NoCollision" :!label _label)
  (switch `/Game/Jason/Enums/En_DoorStatus` (`self.DoorStatus`)
    (:`NewEnumerator0`
      (`FMODBlueprintStatics.PlayEvent2D` "/Game/FMOD/Events/Door/Door_Open_Creak.Door_Open_Creak")
      (set `self.DoorStatus` "NewEnumerator1")
      (bind (_direction _door_float _doorknob_float) (`Timeline|Timeline` :!label _label_2)
        (:`Update`
          (`SceneComponent.K2_SetRelativeRotation` (`self.DOOR`) (`KismetMathLibrary.MakeRotator` 0.0 0.0 _door_float) false false)
          (`SceneComponent.K2_SetRelativeRotation` (`self.HandleScene`) (`KismetMathLibrary.MakeRotator` _doorknob_float) false false))
        (:`Finished`
          (`PrimitiveComponent.SetCollisionEnabled` (`self.DOOR`) "QueryAndPhysics"))))
    (:`NewEnumerator1`
      (`FMODBlueprintStatics.PlayEvent2D` "/Game/FMOD/Events/Door/Door_Wood_Close.Door_Wood_Close")
      (set `self.DoorStatus` "NewEnumerator0")
      (goto _label_2 :!via `Reverse`))))

(event `/Game/Jason/Interface/BPI_InteractInterface.InteractSuccess`
  (params (InteractingCaller :type "Actor Object Reference"))
  (goto _label))

(event `/Game/Jason/Interface/BPI_InteractInterface.InteractFail`
  (params (`Interacting Actor` :type "Actor Object Reference"))
  (`FMODBlueprintStatics.PlayEventAtLocation` "/Game/FMOD/Events/Door/Door_Knob_Rattle.Door_Knob_Rattle" (`KismetMathLibrary.Conv_VectorToTransform` (`self.K2_GetActorLocation` self))))

(fn `CanInteract`
  (params (InteractingActor :type "Actor Object Reference"))
  (returns (CanInteract :type Boolean))
  (bind _doorcolor (`self.DoorColor`))
  (bind _asbp_first_person_character (cast `/Game/FirstPerson/Blueprints/BP_FirstPersonCharacter` InteractingActor))
  (if (== _doorcolor (struct))
    _
    (elif (== (`/Game/FirstPerson/Blueprints/BP_FirstPersonCharacter.KeycardColor` _asbp_first_person_character) _doorcolor)
      _
      (else
        (return false))))
  (return true))

(fn `CloseDoor`
  (params (NewParam :type "/Game/Jason/Enums/En_DoorStatus Enum" :default "NewEnumerator0"))
  (set `self.DoorStatus` "NewEnumerator1")
  (set `self.DoorColor` (struct :`TagName` "SweetSpot.KeyCard.Color.Lock"))
  (`self.LockDoor`))

(fn `OpenDoor`
  (set `self.DoorStatus` "NewEnumerator0")
  (`self.LockDoor`))

(fn `UserConstructionScript`
  (switch `/Game/Haneul/DoorNumber` (`self.Number`)
    (:`NewEnumerator0`
      (`StaticMeshComponent.SetStaticMesh` (`self.NamePlate_301`) "/Game/Game/Art/Environments/Man-Made/Props/Furniture/NamePlate_301.NamePlate_301"))
    (:`NewEnumerator1`
      (`StaticMeshComponent.SetStaticMesh` (`self.NamePlate_301`) "/Game/Game/Art/Environments/Man-Made/Props/Furniture/NamePlate_302.NamePlate_302"))
    (:`NewEnumerator2`
      (`StaticMeshComponent.SetStaticMesh` (`self.NamePlate_301`) "/Game/Game/Art/Environments/Man-Made/Props/Furniture/NamePlate_303.NamePlate_303"))
    (:`NewEnumerator3`
      (`StaticMeshComponent.SetStaticMesh` (`self.NamePlate_301`) "/Game/Game/Art/Environments/Man-Made/Props/Furniture/NamePlate_304.NamePlate_304"))
    (:`NewEnumerator4`
      (`StaticMeshComponent.SetStaticMesh` (`self.NamePlate_301`) "/Game/Game/Art/Environments/Man-Made/Props/Furniture/NamePlate_305.NamePlate_305"))
    (:`NewEnumerator5`
      (`StaticMeshComponent.SetStaticMesh` (`self.NamePlate_301`) "/Game/Game/Art/Environments/Man-Made/Props/Furniture/NamePlate_306.NamePlate_306"))))