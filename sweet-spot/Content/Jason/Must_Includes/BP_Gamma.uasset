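; BP_Gamma is a post-process actor that sets up a dynamic material for gamma adjustment.
; Its construction script creates the material instance and assigns it as a full-weight blendable on the PostProcess settings.
; BeginPlay fetches BP_GameInstance but only writes its Gamma value back to itself.
; The node that would set the material's Gamma parameter is disconnected, so this Blueprint never applies the stored value.
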(event `self.ReceiveBeginPlay`
  (`parent.ReceiveBeginPlay`)
  (bind _asbp_game_instance (cast `/Game/Game/BP_GameInstance` (`GameplayStatics.GetGameInstance`)))
  (set `/Game/Game/BP_GameInstance.Gamma` (`/Game/Game/BP_GameInstance.Gamma` _asbp_game_instance) _asbp_game_instance))

(fn `UserConstructionScript`
  (`parent.UserConstructionScript`)
  (bind _returnvalue (`KismetMaterialLibrary.CreateDynamicMaterialInstance` null "Gamma"))
  (set `self.Gamma MAT` _returnvalue)
  (set `PostProcessComponent.Settings` (make `PostProcessSettings` :`WeightedBlendables` (make `WeightedBlendables` (`|MakeArray` (make `WeightedBlendable` 1.0 (`self.Gamma MAT`))))) (`self.PostProcess`)))