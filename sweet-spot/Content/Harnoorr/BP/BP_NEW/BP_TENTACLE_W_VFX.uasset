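; Tentacle actor that procedurally animates a skeletal mesh through a Control Rig component, giving it organic, wandering motion.
; On rig pre-initialization it maps the mesh as the rig's output and randomizes a noise offset vector for each Offsets entry.
; A looping timer at roughly 60 Hz adds time-based, per-axis Perlin noise to each named control's current local position, so movement accumulates rather than oscillating around a stored rest pose.
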(event `self.ControlRig.OnPreInitializeDelegate`
  (params (Component :type "ControlRigComponent Object Reference"))
  (bind _offsets (`self.Offsets`))
  (`ControlRigComponent.AddMappedCompleteSkeletalMesh` Component (`self.SkeletalMesh`) "Output")
  (for (_ _array_index) _offsets
    (`KismetArrayLibrary.Array_Set` _offsets _array_index (* (`KismetMathLibrary.RandomUnitVector`) (10.0 10.0 10.0)))))

(event `self.ReceiveBeginPlay`
  (`KismetSystemLibrary.K2_SetTimerDelegate` (delegate `TentacleMoving`) 0.016 true))

(event `TentacleMoving`
  (bind _returnvalue (* (`KismetSystemLibrary.GetGameTimeInSeconds`) 1.0))
  (for (_array_element _array_index) (`self.ControlNames`)
    (bind _output_x (`KismetMathLibrary.BreakVector` (`|GetArrayItem` (`self.Offsets`) _array_index)))
    (bind (_output_x_2 _output_y) (`KismetMathLibrary.BreakVector` (`|GetArrayItem` (`self.Offsets`) _array_index)))
    (bind (_output_x_3 _output_y_2 _output_z) (`KismetMathLibrary.BreakVector` (`|GetArrayItem` (`self.Offsets`) _array_index)))
    (`ControlRigComponent.SetControlPosition` (`self.ControlRig`) _array_element (+ (`ControlRigComponent.GetControlPosition` (`self.ControlRig`) _array_element "LocalSpace") (`KismetMathLibrary.MakeVector` (`KismetMathLibrary.PerlinNoise1D` (+ _returnvalue _output_x)) (`KismetMathLibrary.PerlinNoise1D` (+ _returnvalue _output_y)) (`KismetMathLibrary.PerlinNoise1D` (+ _returnvalue _output_z)))) "LocalSpace")))

(fn `UserConstructionScript`)