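; BP_PromptPopUp is a one-shot trigger actor that shows an instruction image pop-up when the first-person character's capsule overlaps it.
; On overlap it optionally enables the character's AllowFocus flag, then disables its own collision to prevent retriggering.
; It fetches the WBP_PopUp widget from PlayerHud, waits a configurable delay, calls Prompt with its image and destroys itself.
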(event `self.CollisionComponent.OnComponentBeginOverlap`
  (params (OverlappedComponent :type "PrimitiveComponent Object Reference") (OtherActor :type "Actor Object Reference") (OtherComp :type "PrimitiveComponent Object Reference") (OtherBodyIndex :type Integer) (bFromSweep :type Boolean) (SweepResult :type "HitResult Structure (by ref)"))
  (cast `CapsuleComponent` OtherComp)
  (bind _asbp_first_person_character (cast `/Game/FirstPerson/Blueprints/BP_FirstPersonCharacter` OtherActor))
  (if (`self.AllowFocus`)
    (set `/Game/FirstPerson/Blueprints/BP_FirstPersonCharacter.allowFocus` true _asbp_first_person_character))
  (`PrimitiveComponent.SetCollisionEnabled` (`self.CollisionComponent`) "NoCollision")
  (bind _asplayer_hud (cast `PlayerHud` (`PlayerController.GetHUD` (`GameplayStatics.GetPlayerController` 0))))
  (bind _aswbp_pop_up (cast `/Game/Haneul/Widget/WBP_PopUp` (`PlayerHud.PopUpWidget` _asplayer_hud)))
  (`KismetSystemLibrary.Delay` (`self.DelayTime`))
  (`/Game/Haneul/Widget/WBP_PopUp.Prompt` _aswbp_pop_up (`self.Img`) true (1.538 1.0))
  (`self.K2_DestroyActor`))

(fn `UserConstructionScript`)