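; Tentacle wall actor that spawns a BP_TENTACLE on its static mesh at BeginPlay and disables a linked Prompt's collision.
; CameraShake starts a focus shake and sets the tentacle's custom depth stencil, likely for highlighting, when Count is zero; ResetTentaclePosition only reverts both effects.
; DestroyTentacle, also called on EndPlay, opens the linked Door, restores Prompt collision and destroys the tentacle and wall.
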(event `self.ReceiveBeginPlay`
  (bind _prompt (`self.Prompt`))
  (bind _returnvalue (`|SpawnActorFromClass` "/Game/Harnoorr/BP/BP_NEW/BP_TENTACLE.BP_TENTACLE_C" (`SceneComponent.K2_GetComponentToWorld` (`self.StaticMesh`)) "AlwaysSpawn" "MultiplyWithRoot" null null))
  (bind _output_get (set `self.Tentacle` _returnvalue))
  (`self.K2_AttachToComponent` _output_get (`self.StaticMesh`) "None" "SnapToTarget" "SnapToTarget" "KeepRelative" true)
  (`PrimitiveComponent.SetRenderCustomDepth` (`/Game/Harnoorr/BP/BP_NEW/BP_TENTACLE.SkeletalMesh` (`self.Tentacle`)) true)
  (`/Engine/EditorBlueprintResources/StandardMacros.IsValid` _prompt
    (:`Is Valid`
      (`PrimitiveComponent.SetCollisionEnabled` (`TriggerBase.CollisionComponent` _prompt) "NoCollision"))))

(event `self.DestroyTentacle`
  (bind _door (`self.Door`))
  (bind _tentacle (`self.Tentacle`))
  (bind _prompt (`self.Prompt`))
  (`/Engine/EditorBlueprintResources/StandardMacros.IsValid` _door
    (:`Is Valid`
      (`/Game/Harnoorr/BP/BP_NEW/BP_NEW_DOOR_COPY.OpenDoor` _door))
    (:`Is Not Valid`
      _))
  (`/Engine/EditorBlueprintResources/StandardMacros.IsValid` _prompt
    (:`Is Valid`
      (`PrimitiveComponent.SetCollisionEnabled` (`TriggerBase.CollisionComponent` _prompt) "QueryAndPhysics"))
    (:`Is Not Valid`
      _))
  (`/Engine/EditorBlueprintResources/StandardMacros.IsValid` _tentacle
    (:`Is Valid`
      (`self.K2_DestroyActor` _tentacle))
    (:`Is Not Valid`
      _))
  (`self.K2_DestroyActor`))

(event `self.CameraShake`
  (if (== (`self.count`) 0)
    (`PlayerCameraManager.StartCameraShake` :`self` (`GameplayStatics.GetPlayerCameraManager` 0) :`ShakeClass` "/Game/Haneul/CameraShake/BP_CamShakeFocus.BP_CamShakeFocus_C")
    (`PrimitiveComponent.SetCustomDepthStencilValue` (`/Game/Harnoorr/BP/BP_NEW/BP_TENTACLE.SkeletalMesh` (`self.Tentacle`)) 1)))

(event `self.ResetTentaclePosition`
  (`PlayerCameraManager.StopAllCameraShakes` (`GameplayStatics.GetPlayerCameraManager` 0) true)
  (`PrimitiveComponent.SetCustomDepthStencilValue` (`/Game/Harnoorr/BP/BP_NEW/BP_TENTACLE.SkeletalMesh` (`self.Tentacle`)) 0))

(event `self.ReceiveEndPlay`
  (params (EndPlayReason :type "EEndPlayReason Enum" :default "Destroyed"))
  (`self.Destroy Tentacle`))

(fn `Destroy Tentacle`
  (bind _tentacle (`self.Tentacle`))
  (`/Engine/EditorBlueprintResources/StandardMacros.IsValid` _tentacle
    (:`Is Valid`
      (`self.K2_DestroyActor` _tentacle))
    (:`Is Not Valid`
      _))
  (`self.K2_DestroyActor`))

(fn `UserConstructionScript`)