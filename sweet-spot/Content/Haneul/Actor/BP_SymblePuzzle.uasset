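; BP_SymblePuzzle is an interactable symbol in an ordered puzzle chain that rewards the player with an elevator part.
; Interacting with the active symbol activates the next one, or grants the part at the chain's end, then plays a sound and destroys the actor.
; An inactive symbol instead raises the HUD madness bar, shakes the camera, plays an audio event and briefly flashes a jump-scare widget.
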(event `self.ReceiveBeginPlay`
  (bind _returnvalue (`|CreateWidget` "/Game/Haneul/Widget/WBP_JumpScare.WBP_JumpScare_C"))
  (bind _output_get (set `self.redFlashWidget` _returnvalue))
  (`UserWidget.AddToViewport` _output_get 0)
  (set `Widget.Visibility` "Hidden" (`self.redFlashWidget`)))

(event `/Game/Jason/Interface/BPI_InteractInterface.InteractSuccess`
  (params (InteractingCaller :type "Actor Object Reference"))
  (bind _nextsymblepuzzle (`self.nextSymblePuzzle`))
  (if (`self.isActive`)
    (`/Engine/EditorBlueprintResources/StandardMacros.IsValid` _nextsymblepuzzle
      (:`Is Valid`
        (set `SymblePuzzle.isActive` true _nextsymblepuzzle)
        (`FMODBlueprintStatics.PlayEventAtLocation` "/Game/FMOD/Events/UI/ButtonMouseOver.ButtonMouseOver" (`KismetMathLibrary.Conv_VectorToTransform` (`self.K2_GetActorLocation` self))))
      (:`Is Not Valid`
        (bind _asbp_first_person_character (cast `/Game/FirstPerson/Blueprints/BP_FirstPersonCharacter` (`Controller.K2_GetPawn` (`GameplayStatics.GetPlayerController` 0))))
        (`PlayerInventory.GetElevatorPart` (`/Game/FirstPerson/Blueprints/BP_FirstPersonCharacter.PlayerInventory` _asbp_first_person_character) (`self.ElevatorPart`))
        (`FMODBlueprintStatics.PlayEventAtLocation` "/Game/FMOD/Events/UI/ButtonPress.ButtonPress" (`KismetMathLibrary.Conv_VectorToTransform` (`self.K2_GetActorLocation` self)))))
    (`self.K2_DestroyActor`)
    (else
      (`self.IncreaseMadness`)
      (`self.CameraShake`)
      (`FMODBlueprintStatics.PlayEventAtLocation` null (`KismetMathLibrary.Conv_VectorToTransform` (`self.K2_GetActorLocation` self)))
      (set `Widget.Visibility` "Visible" (`self.redFlashWidget`))
      (`KismetSystemLibrary.Delay` 0.2)
      (set `Widget.Visibility` "Hidden" (`self.redFlashWidget`)))))

(fn `CameraShake`
  (`GameplayStatics.PlayWorldCameraShake` null (`self.K2_GetActorLocation` (`Controller.K2_GetPawn` (`GameplayStatics.GetPlayerController` 0))) 0.0 1000.0))

(fn `CanInteract`
  (params (InteractingActor :type "Actor Object Reference"))
  (returns (CanInteract :type Boolean))
  (cast `/Game/FirstPerson/Blueprints/BP_FirstPersonCharacter` InteractingActor)
  (return true))

(fn `IncreaseMadness`
  (bind _asplayer_hud (cast `PlayerHud` (`PlayerController.GetHUD` (`GameplayStatics.GetPlayerController` 0))))
  (bind _asbp_madness_bar (cast `/Game/Jason/UI/Blueprints/BP_MadnessBar` (`PlayerHud.GetMadnessMeterWidget` _asplayer_hud)))
  (`MyUserWidget.IncreaseMadnessBar` _asbp_madness_bar (`self.Increase Madness`)))

(fn `UserConstructionScript`)